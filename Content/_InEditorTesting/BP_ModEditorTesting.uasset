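; BP_ModEditorTesting is an in-editor test actor that sets up a player environment for testing mods.
; On BeginPlay it creates a hit-indicator widget, waits for the SBZ player character, assigns player state and character data, then spawns enabled mod actors from a class map.
; An optional fake head mask hides in first person through a camera-mode callback.
; Debug prints report setup and, each tick, a camera-manager child component.
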(event `self.ReceiveBeginPlay`
  (`|CreateWidget` "/Script/Starbreeze.SBZHUDHitIndicatorWidget")
  (bind _assbzplayer_character (`/Game/Mods/_LesnovMods/BML_Actor.ValidCheck(Wait | SBZPlayerCharacter)`))
  (set `self.As SBZPlayer Character` _assbzplayer_character)
  (bind _assbzplayer_state (cast `SBZPlayerState` (`Controller.PlayerState` (`Pawn.GetController` _assbzplayer_character))))
  (bind _output_get (set `SBZPlayerCharacter.SBZPlayerState` _assbzplayer_state _assbzplayer_character))
  (`self.DebugText` (`KismetStringLibrary.Concat_StrStr` (`KismetSystemLibrary.GetDisplayName` _output_get) " - Player State Obtained"))
  (set `SBZPlayerState.CurrentCharacterData` (`self.Current Character Data`) _assbzplayer_state)
  (`self.AddFakeMask` (`self.Add Fake Mask`))
  (bind _asfirst_person_character (cast `/Game/_InEditorTesting/FirstPersonBP/Blueprints/FirstPersonCharacter` (`self.As SBZPlayer Character`)))
  (add `/Game/_InEditorTesting/FirstPersonBP/Blueprints/FirstPersonCharacter.OnCameraModeChanged` _asfirst_person_character (`|CreateDelegate` :!event `OnCameraModeChanged_Event_0`))
  (`self.NewFunction_0`))

(event `self.ReceiveTick`
  (params (DeltaSeconds :type "Float (single-precision)"))
  (`KismetSystemLibrary.PrintString` (`KismetSystemLibrary.GetDisplayName` (`SceneComponent.GetChildComponent` (`Actor.RootComponent` (`GameplayStatics.GetPlayerCameraManager` 0)) 0))))

(event `OnCameraModeChanged_Event_0`
  (params (IsFirstPerson :type Boolean))
  (bind _equippedmask (`SBZCharacter.EquippedMask` (`self.As SBZPlayer Character`)))
  (`/Engine/EditorBlueprintResources/StandardMacros.IsValid` _equippedmask
    (:`Is Valid`
      (`self.SetActorHiddenInGame` _equippedmask IsFirstPerson)
      (`KismetSystemLibrary.PrintString` (`KismetStringLibrary.Conv_BoolToString` IsFirstPerson) true true (struct :`R` 1.0 :`B` 0.030596 :`A` 1.0)))))

(fn `AddFakeMask`
  (params (AddFakeMask :type Boolean))
  (if AddFakeMask
    (bind _returnvalue (`|SpawnActorFromClass` "/Game/_InEditorTesting/BP_FakeMask.BP_FakeMask_C" (`KismetMathLibrary.MakeTransform` (0.0 0.0 0.0)) "AlwaysSpawn" "OverrideRootScale" null null))
    (`self.K2_AttachToComponent` _returnvalue (`Character.Mesh` (`self.As SBZPlayer Character`)) "Head" "SnapToTarget" "SnapToTarget" "SnapToTarget" true)
    (bind _output_get (set `SBZCharacter.EquippedMask` _returnvalue (`self.As SBZPlayer Character`)))
    (`self.SetActorHiddenInGame` _output_get true)))

(fn `DebugText`
  (params (B :type String))
  (`KismetSystemLibrary.PrintString` (`KismetStringLibrary.Concat_StrStr` "[EditorTesting] " B) true true (struct :`G` 1.0 :`B` 0.11576 :`A` 1.0) 5.0))

(fn `NewFunction_0`
  (bind _class (`self.Class`))
  (bind _keys (`BlueprintMapLibrary.Map_Keys` _class))
  (for _array_element _keys
    (bind (_value _returnvalue) (`BlueprintMapLibrary.Map_Find` _class _array_element))
    (if (and _value _returnvalue)
      (`self.DebugText` (`KismetStringLibrary.Concat_StrStr` "ModActorSpawned - " (`KismetSystemLibrary.GetClassDisplayName` _array_element)))
      (`|SpawnActorFromClass` _array_element (`KismetMathLibrary.MakeTransform` (0.0 0.0 0.0)) "AlwaysSpawn" "OverrideRootScale" null null))))

(fn `UserConstructionScript`)