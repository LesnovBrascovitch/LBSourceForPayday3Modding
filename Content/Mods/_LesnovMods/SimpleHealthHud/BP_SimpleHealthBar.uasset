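; Mod actor that shows a HUD health and armor bar for the AI character the local player is looking at.
; On BeginPlay it creates the bar widget, retries until the SBZ player pawn exists, and rebinds when that pawn is destroyed.
; A looping timer traces from the first-person camera and feeds the hit AI's attributes to the widget, hiding it otherwise.
; Unpackaged builds run a test routine with dummy values instead.
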(event `OnDestroyed_Event_0`
  (params (DestroyedActor :type "Actor Object Reference"))
  (bind _menu_healthbar (`self.Menu_HealthBar`))
  (bind _assbzplayer_character (cast `SBZPlayerCharacter` (`SBZPlayerLibrary.GetLocalPlayerPawn`) :!label _label)
    (:`then`
      (bind _output_get (set `self.As SBZPlayer Character` _assbzplayer_character))
      (set `self.FPCamera Attachment` (`SBZPlayerCharacter.FPCameraAttachment` _output_get))
      (`KismetSystemLibrary.K2_SetTimerDelegate` (delegate `CustomEvent_0`) 0.2 true)
      (`Widget.SetVisibility` (`self.Menu_HealthBar`) "Collapsed")
      (add `Actor.OnDestroyed` (`self.As SBZPlayer Character`) (delegate `OnDestroyed_Event_0`)))
    (:`CastFailed`
      (`/Game/Mods/_LesnovMods/SimpleHealthHud/Menu_SimpleHealthBar.SetText` _menu_healthbar "SBZPlayer Casting Failed")
      (`Widget.SetVisibility` _menu_healthbar "Collapsed")
      (`KismetSystemLibrary.Delay` 0.2)
      (goto _label))))

(event `self.ReceiveBeginPlay`
  (bind _menu_healthbar (`self.Menu_HealthBar`))
  (`parent.ReceiveBeginPlay`)
  (bind _returnvalue (`|CreateWidget` "/Game/Mods/_LesnovMods/SimpleHealthHud/Menu_SimpleHealthBar.Menu_SimpleHealthBar_C"))
  (`UserWidget.AddToViewport` _returnvalue 0)
  (set `self.Menu_HealthBar` _returnvalue)
  (`Widget.SetVisibility` (`self.Menu_HealthBar`) "Collapsed")
  (if (`KismetSystemLibrary.IsPackagedForDistribution`)
    (goto _label)
    (else
      (`Widget.SetVisibility` (`self.Menu_HealthBar`) "SelfHitTestInvisible")
      (`/Game/Mods/_LesnovMods/SimpleHealthHud/Menu_SimpleHealthBar.SetHealth` _menu_healthbar 15.0 777.0)
      (`/Game/Mods/_LesnovMods/SimpleHealthHud/Menu_SimpleHealthBar.SetArmor` _menu_healthbar 155.0 333.0)
      (`KismetSystemLibrary.Delay` 2.0)
      (`/Game/Mods/_LesnovMods/SimpleHealthHud/Menu_SimpleHealthBar.SetArmor` _menu_healthbar 0.0 0.0))))

(event `CustomEvent_0`
  (bind _fpcamera_attachment (`self.FPCamera Attachment`))
  (bind _menu_healthbar (`self.Menu_HealthBar`))
  (bind _returnvalue (`SceneComponent.K2_GetComponentLocation` _fpcamera_attachment))
  (bind (_outhit _returnvalue_2) (`KismetSystemLibrary.LineTraceSingle` _returnvalue (+ _returnvalue (* (`SceneComponent.GetForwardVector` _fpcamera_attachment) 30000)) "TraceTypeQuery2" false (`|MakeArray` (`self.As SBZPlayer Character`) :!type "Actor Object Reference")))
  (if _returnvalue_2
    (bind (_bblockinghit _binitialoverlap _time _distance _location _impactpoint _normal _impactnormal _physmat _hitactor) (`GameplayStatics.BreakHitResult` _outhit))
    (if (`KismetMathLibrary.ClassIsChildOf` (`GameplayStatics.GetObjectClass` _hitactor) "/Script/Starbreeze.SBZAIBaseCharacter")
      (bind _assbzaibase_character (cast `SBZAIBaseCharacter` _hitactor)
        (:`then`
          (`Widget.SetVisibility` (`self.Menu_HealthBar`) "SelfHitTestInvisible")
          (bind _attributeset (`SBZAIBaseCharacter.AttributeSet` _assbzaibase_character))
          (bind (_health_basevalue _health_currentvalue) (break `GameplayAttributeData` (`SBZPawnAttributeSet.Health` _attributeset)))
          (bind (_healthmax_basevalue _healthmax_currentvalue) (break `GameplayAttributeData` (`SBZPawnAttributeSet.HealthMax` _attributeset)))
          (`/Game/Mods/_LesnovMods/SimpleHealthHud/Menu_SimpleHealthBar.SetHealth` _menu_healthbar _health_currentvalue _healthmax_currentvalue)
          (bind _attributeset_2 (`SBZAIBaseCharacter.AttributeSet` _assbzaibase_character))
          (bind (_armor_basevalue _armor_currentvalue) (break `GameplayAttributeData` (`SBZPawnAttributeSet.Armor` _attributeset_2)))
          (bind (_armormax_basevalue _armormax_currentvalue) (break `GameplayAttributeData` (`SBZPawnAttributeSet.ArmorMax` _attributeset_2)))
          (`/Game/Mods/_LesnovMods/SimpleHealthHud/Menu_SimpleHealthBar.SetArmor` _menu_healthbar _armor_currentvalue _armormax_currentvalue))
        (:`CastFailed`
          (`Widget.SetVisibility` (`self.Menu_HealthBar`) "Hidden" :!label _label_2)))
      (else
        (goto _label_2)))
    (else
      (goto _label_2))))

(fn `UserConstructionScript`
  (`parent.UserConstructionScript`))