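; Damage popup mod actor that spawns floating damage numbers above victims hit by the local player character.
; It binds to the game event broker's damage event, passing damage, critical, killshot, armor and distance-scaled font size to BP_FloatingText_Damage.
; When the player character is destroyed, it reacquires the character and rebinds to keep popups working after respawn.
; An editor-only testing path spawns randomized popups on a looping timer.
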(event `OnTakenDamage_Event_0`
  (params (DamageEventData :type "SBZDamageEvent Structure (by ref)"))
  (bind (_attacker _causer _victim _equippabledata _throwabledata _damage _armordamage _healthdamage _bcritical _bwasarmorbroken _biskillshot) (break `SBZDamageEvent` DamageEventData))
  (if (== _attacker (`self.As SBZPlayer Character`))
    (`|SpawnActorFromClass` "/Game/Mods/_LesnovMods/DamagePopup/BP_FloatingText_Damage.BP_FloatingText_Damage_C" (`KismetMathLibrary.MakeTransform` (+ (`self.K2_GetActorLocation` _victim) (0.0 0.0 50.0))) "AlwaysSpawn" "OverrideRootScale" null (`KismetMathLibrary.FTrunc` _damage) _bcritical _biskillshot (> _armordamage 0.0) (`KismetMathLibrary.MapRangeClamped` (`self.GetDistanceTo` _attacker _victim) (`self.In Range A`) (`self.In Range B`) 1.0 3.0) (struct :`R` 1.0 :`G` 1.0 :`B` 1.0 :`A` 1.0) null)))

(event `CustomEvent_0`
  (`|SpawnActorFromClass` "/Game/Mods/_LesnovMods/DamagePopup/BP_FloatingText_Damage.BP_FloatingText_Damage_C" (`KismetMathLibrary.MakeTransform` (`self.K2_GetActorLocation` (`self.InEditorTesting`))) "Undefined" "OverrideRootScale" null (`KismetMathLibrary.RandomIntegerInRange` 0 1111) (`KismetMathLibrary.RandomBool`) (`KismetMathLibrary.RandomBool`) (`KismetMathLibrary.RandomBool`) (`KismetMathLibrary.MapRangeClamped` (`KismetMathLibrary.RandomFloatInRange` 0.0 1000.0) 300.0 1000.0 1.0 3.0) (struct :`R` 1.0 :`G` 1.0 :`B` 1.0 :`A` 1.0) null))

(event `self.ReceiveBeginPlay`
  (`parent.ReceiveBeginPlay`)
  (`/Game/Mods/_LesnovMods/BML_Actor.IsInEditor`
    (:`InEditor`
      (`KismetSystemLibrary.K2_SetTimerDelegate` (delegate `CustomEvent_0`) 0.5 true))
    (:`InGame`
      (bind _assbzplayer_character (`/Game/Mods/_LesnovMods/BML_Actor.ValidCheck(Wait | SBZPlayerCharacter)` :!label _label))
      (bind _output_get (set `self.As SBZPlayer Character` _assbzplayer_character))
      (bind _returnvalue (`SBZEventLibrary.GetGameEventBroker`))
      (add `SBZGameEventBroker.OnTakenDamage` _returnvalue (delegate `OnTakenDamage_Event_0`))
      (add `self.OnDestroyed` _output_get (delegate `OnDestroyed_Event_0`)))))

(event `OnDestroyed_Event_0`
  (params (DestroyedActor :type "Actor Object Reference"))
  (goto _label))

(fn `UserConstructionScript`
  (`parent.UserConstructionScript`))