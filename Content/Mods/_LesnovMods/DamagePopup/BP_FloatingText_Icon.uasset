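; Floating damage-popup actor that shows status text through its UI_DamageText_Base widget, with killshot, critical and armor flags, and rises straight up before destroying itself.
; BeginPlay derives a fixed per-cycle step from travel distance and speed, which the UpdateWidgetLocation override applies along Z.
; Distance covered is computed from the parent's update iteration count, deciding both destruction and when peak widget scale is passed.
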(event `self.ReceiveBeginPlay`
  ;[0 1 0 0.5] Initialization Protocols
  (bind _asui_damage_text_base (cast `/Game/Mods/_LesnovMods/DamagePopup/UI_DamageText_Base` (`WidgetComponent.GetUserWidgetObject` (`self.TextWidget`))))
  (`/Game/Mods/_LesnovMods/DamagePopup/UI_DamageText_Base.SetDisplayText` _asui_damage_text_base (`self.StatusText`) (`self.Is Killshot`) (`self.Critical`) (`self.Is Armor`) 0.0)
  ;;[1 1 1] Sets movement constraints for the linear motion
  (set `self.VerticalDisplacementPerCycle` (* (`self.DistanceToCover`) (`self.MovementSpeedController`)))
  (`parent.ReceiveBeginPlay`))

(event `self.RunUpdateCycle`
  ;[0 1 1 0.5] Updates the floating text state
  (`parent.RunUpdateCycle`)
  (if (>= (`self.GetVerticalDistanceCovered`) (`self.DistanceToCover`))
    (`self.K2_DestroyActor`)))

(event `self.UpdateWidgetLocation`
  (bind (_returnvalue_x _returnvalue_y _returnvalue_z) (`KismetMathLibrary.BreakVector` (`self.K2_GetActorLocation`)))
  ;[0 1 1 0.5] Updates the floating text state
  (`self.K2_SetActorLocation` (`KismetMathLibrary.MakeVector` _returnvalue_x _returnvalue_y (+ _returnvalue_z (`self.VerticalDisplacementPerCycle`)))))

(fn `GetVerticalDistanceCovered`
  (returns (ReturnValue :type "Float (double-precision)"))
  (return (* (`self.UpdateIteration`) (`KismetMathLibrary.Abs` (`self.VerticalDisplacementPerCycle`)))))

(fn `ReachedPointOfMaxWidgetScale?`
  (returns (`Yes?` :type Boolean))
  (return (> (`self.GetVerticalDistanceCovered`) (* (`self.DistanceToCover`) (`self.%DistanceToPointOfMaxScale`)))))

(fn `UserConstructionScript`)