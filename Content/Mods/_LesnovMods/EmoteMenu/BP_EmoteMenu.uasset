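; Emote menu mod actor that lets the local player pick and play emotes with music and a dedicated camera.
; Loads EmoteSettings assets by path into eight-slot wheel pages, toggled with key 5.
; Selection hides the weapon and swaps the mesh to ABP_Emote; damage or a non-loop timer disables the camera, and finishing restores the cached anim class.
; Key J opens per-emote volume settings, persisted in EmoteSavegame.
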(event `self.ReceiveBeginPlay`
  (bind _savegame (`/Game/Mods/_LesnovMods/BML_Object.HandleSaveGame` "/Game/Mods/_LesnovMods/EmoteMenu/EmoteSavegame.EmoteSavegame_C")
    (:`Exec`
      (bind _asemote_savegame (cast `/Game/Mods/_LesnovMods/EmoteMenu/EmoteSavegame` _savegame))
      (set `self.As Emote Savegame` _asemote_savegame)
      ;[1 1 1] Load EmoteSettings data asset by path
      (bind _assetdata (`/Game/Mods/_LesnovMods/BML_Object.LoadAllAssetsByPath` "/Game/Mods/_LesnovMods/EmoteMenu/EmoteAssets")
        (:`LoopBody`
          (bind _asemote_settings (cast `/Game/Mods/_LesnovMods/EmoteMenu/EmoteSettings` _assetdata))
          (`KismetSystemLibrary.PrintString` (`KismetSystemLibrary.GetDisplayName` _asemote_settings))
          (if (and (!= _asemote_settings "/Game/Mods/_LesnovMods/EmoteMenu/EmoteAssets/ES_Empty.ES_Empty") (!= _asemote_settings "/Game/Mods/_LesnovMods/EmoteMenu/EmoteAssets/ES_Testing01.ES_Testing01") (!= _asemote_settings "/Game/Mods/_LesnovMods/EmoteMenu/EmoteAssets/ES_Testing02.ES_Testing02") (!= _asemote_settings "/Game/Mods/_LesnovMods/EmoteMenu/EmoteAssets/Nested/ES_Testing03.ES_Testing03"))
            (`KismetArrayLibrary.Array_AddUnique` (`self.PreLoadedEmoteSettings`) _asemote_settings)))
        (:`Completed`
          (bind _assbzplayer_character (`/Game/Mods/_LesnovMods/BML_Actor.ValidCheck(Wait | SBZPlayerCharacter)`))
          (set `self.As SBZPlayer Character` _assbzplayer_character)
          ;[1 1 1] Comment
          (`self.CreateEmoteMenu`)
          (`/Game/Mods/_LesnovMods/BML_Actor.ToggleInputByLocalController` null true)
          ;[1 1 1] Spawn and Initialize the Emote Camera
          (bind _returnvalue (`|SpawnActorFromClass` "/Game/Mods/_LesnovMods/EmoteMenu/BP_EmoteCamera.BP_EmoteCamera_C" (`KismetMathLibrary.MakeTransform` (0.0 0.0 0.0)) "AlwaysSpawn" "OverrideRootScale" null (`/Game/Mods/_LesnovMods/BML_Actor.GetLocalPlayerController(Comp)`) null))
          (bind _output_get (set `self.EmoteCamera` _returnvalue))
          (add `/Game/Mods/_LesnovMods/EmoteMenu/BP_EmoteCamera.OnEmoteStoppedKeyPressed` _output_get (`|CreateDelegate` :!event `OnEmoteFinished`))
          (`self.LoadEmoteAssets`)
          (`/Game/Mods/_LesnovMods/EmoteMenu/Menu_EM_MainMenu.RefleshBar` (`self.EmoteMenu`))
          ;[1 1 1] INPUT
          (`|SpawnActorFromClass` "/Game/Mods/_LesnovMods/EmoteMenu/INPUT_EmotePageSelection.INPUT_EmotePageSelection_C" (`KismetMathLibrary.MakeTransform` (0.0 0.0 0.0)) "AlwaysSpawn" "OverrideRootScale" null self null)
          (bind _assbzplayer_character_2 (`/Game/Mods/_LesnovMods/BML_Actor.ValidCheck(Wait | SBZPlayerCharacter)` :!label _label))
          (bind _output_get_2 (set `self.As SBZPlayer Character` _assbzplayer_character_2))
          (add `self.OnDestroyed` _output_get_2 (delegate `OnDestroyed_Event_0`))
          (set `self.NewVar_0` (`GameplayStatics.GetObjectClass` (`SkeletalMeshComponent.GetAnimInstance` (`Character.Mesh` (`self.As SBZPlayer Character`)))))
          (`KismetSystemLibrary.K2_SetTimerDelegate` (delegate `Debug`) 0.5 true)
          (`KismetSystemLibrary.Delay` 1.0)
          (`self.NewFunction_0`))))))

(event `CustomEvent_0`
  (params (Target :type "/Game/Mods/_LesnovMods/EmoteMenu/Menu_EM_EmoteWheel Object Reference"))
  (add `/Game/Mods/_LesnovMods/EmoteMenu/Menu_EM_EmoteWheel.OnEmoteSelected` Target (`|CreateDelegate` :!event `OnEmoteSelected_Event_0`)))

(event `OnDestroyed_Event_0`
  (params (DestroyedActor :type "Actor Object Reference"))
  (goto _label))

(event `Debug`
  (`KismetSystemLibrary.PrintString` (`KismetSystemLibrary.GetDisplayName` (`SkeletalMeshComponent.GetAnimInstance` (`Character.Mesh` (`self.As SBZPlayer Character`))))))

(event `OnEmoteSelected_Event_0`
  (params (EmoteSettings :type "/Game/Mods/_LesnovMods/EmoteMenu/EmoteSettings Object Reference"))
  (bind _playercontroller (`/Game/Mods/_LesnovMods/BML_Actor.GetLocalPlayerController(Comp)`))
  (bind _spawnclass (`/Game/Mods/_LesnovMods/EmoteMenu/EmoteSettings.SpawnClass` (`self.Emote Settings`)))
  ;[1 1 1] OnEmoteSelected Event
  (set `self.Emote Settings` EmoteSettings)
  (`self.Bind`)
  (`KismetSystemLibrary.K2_ClearAndInvalidateTimerHandle` (`self.Timer_AnimStop`))
  (set `self.IsEmoteActivated` true)
  (`self.ToggleVisibillity(FPWeapon)` true)
  (`self.PlayEmoteAnimation`)
  (`/Game/Mods/_LesnovMods/EmoteMenu/BP_EmoteCamera.OnControl` (`self.EmoteCamera`))
  (`self.PlayMusicByEmoteSettings` (`self.Emote Settings`))
  (`self.ToggleEmoteMenuVisibillity` false)
  (set `PlayerController.bShowMouseCursor` false _playercontroller)
  (`WidgetBlueprintLibrary.SetInputMode_GameOnly` _playercontroller)
  (if (`KismetSystemLibrary.IsValidClass` _spawnclass)
    (`|SpawnActorFromClass` _spawnclass (`KismetMathLibrary.MakeTransform` (`self.K2_GetActorLocation` (`self.As SBZPlayer Character`))) "AlwaysSpawn" "OverrideRootScale" null null)))

(event `OnEmoteFinished`
  ;[1 1 1] OnEmoteFInished Event
  (`KismetSystemLibrary.K2_ClearAndInvalidateTimerHandle` (`self.Timer_AnimStop`))
  (`self.Unbind`)
  (`self.ToggleEmoteMenuVisibillity` false)
  (`self.ToggleVisibillity(FPWeapon)` false)
  (set `self.IsEmoteActivated` false)
  (`/Game/Mods/_LesnovMods/BML_Actor.ToggleMouseCursor` false)
  (`self.OnEmoteMenuClosed`)
  (`WidgetBlueprintLibrary.SetInputMode_GameOnly` (`/Game/Mods/_LesnovMods/BML_Actor.GetLocalPlayerController(Comp)`))
  (`self.StopMusic`)
  (`SkeletalMeshComponent.SetAnimInstanceClass` (`Character.Mesh` (`self.As SBZPlayer Character`)) (`self.NewVar_0`)))

(event `CloseEmoteMenu`
  (bind _emotemenu (`self.EmoteMenu`))
  (`/Engine/EditorBlueprintResources/StandardMacros.IsValid` _emotemenu
    (:`Is Valid`
      (if (`Widget.IsVisible` _emotemenu)
        ;[1 1 1] Opem Emote Menu
        (`WidgetBlueprintLibrary.SetInputMode_GameOnly` (`/Game/Mods/_LesnovMods/BML_Actor.GetLocalPlayerController(Comp)`) :!label _label_2)
        (`/Game/Mods/_LesnovMods/EmoteMenu/Menu_EM_MainMenu.PlayCloseAnimation` (`self.EmoteMenu`))
        (if (not (`self.IsEmoteActivated`))
          (`self.OnEmoteMenuClosed`))))))

(event `Key|Five` :consume false
  (params (Key :type "Key Structure"))
  ;[1 1 1] Opem Emote Menu
  (:`Pressed`
    (if (`Widget.IsVisible` (`self.EmoteMenu`))
      (`/Game/Mods/_LesnovMods/BML_Actor.ToggleMouseCursor` false)
      (goto _label_2)
      (else
        (`Widget.SetVisibility` (`self.EmoteMenu`) "SelfHitTestInvisible")
        (`/Game/Mods/_LesnovMods/BML_Actor.ToggleMouseCursor` true)
        (`WidgetBlueprintLibrary.SetInputMode_GameAndUIEx` (`/Game/Mods/_LesnovMods/BML_Actor.GetLocalPlayerController(Comp)`) (`self.EmoteMenu`))
        (`/Game/Mods/_LesnovMods/EmoteMenu/Menu_EM_MainMenu.PlayOpenAnimation` (`self.EmoteMenu`))
        (`self.OnEmoteMenuOpened`)
        (`self.CloseSettingMenu`)))))

(event `OnEmotePageIncrement`
  (bind _emotemenu (`self.EmoteMenu`))
  (bind _widgetswitcher_51 (`/Game/Mods/_LesnovMods/EmoteMenu/Menu_EM_MainMenu.WidgetSwitcher_51` (`self.EmoteMenu`)))
  ;[1 1 1] Change Emote Menu's pages (Receive events from INPUT_EmotePageSelection)
  (`WidgetSwitcher.SetActiveWidgetIndex` _widgetswitcher_51 (+ (`WidgetSwitcher.GetActiveWidgetIndex` _widgetswitcher_51) 1))
  (`/Game/Mods/_LesnovMods/EmoteMenu/Menu_EM_MainMenu.RefleshBar` _emotemenu :!label _label_3)
  (`/Game/Mods/_LesnovMods/EmoteMenu/Menu_EM_MainMenu.PlaySwitchAnim` _emotemenu))

(event `OnEmotePageDecrement`
  (bind _widgetswitcher_51 (`/Game/Mods/_LesnovMods/EmoteMenu/Menu_EM_MainMenu.WidgetSwitcher_51` (`self.EmoteMenu`)))
  ;[1 1 1] Change Emote Menu's pages (Receive events from INPUT_EmotePageSelection)
  (`WidgetSwitcher.SetActiveWidgetIndex` _widgetswitcher_51 (- (`WidgetSwitcher.GetActiveWidgetIndex` _widgetswitcher_51) 1))
  (goto _label_3))

(event `StartAnimStopTimer`
  (params (NewParam :type "Float (double-precision)"))
  ;[1 1 1] Stop emote automatically when it is not checked with "is anim looped"
  (bind _returnvalue (`KismetSystemLibrary.K2_SetTimerDelegate` (delegate `SendOnEmoteCameraDisabled`) NewParam))
  (set `self.Timer_AnimStop` _returnvalue)
  (`KismetSystemLibrary.PrintString` (`KismetStringLibrary.Conv_DoubleToString` NewParam)))

(event `Bind`
  (add `self.OnTakeAnyDamage` (`self.As SBZPlayer Character`) (delegate `OnTakeAnyDamage_Event_0`)))

(event `SendOnEmoteCameraDisabled`
  ;[1 1 1] Stop emote automatically when it is not checked with "is anim looped"
  (`/Game/Mods/_LesnovMods/EmoteMenu/BP_EmoteCamera.OnEmoteCameraDisabled` (`self.EmoteCamera`)))

(event `Unbind`
  (remove `self.OnTakeAnyDamage` (`self.As SBZPlayer Character`) (delegate `OnTakeAnyDamage_Event_0`)))

(event `CustomEvent_1`
  (params (MontageToPlay :type "AnimMontage Object Reference") (EmoteSettings :type "/Game/Mods/_LesnovMods/EmoteMenu/EmoteSettings Object Reference"))
  (bind _mesh (`Character.Mesh` (`self.As SBZPlayer Character`)))
  (`SkeletalMeshComponent.SetAnimInstanceClass` _mesh "/Game/Mods/_LesnovMods/EmoteMenu/ABP_Emote.ABP_Emote_C")
  (`|PlayMontage` _mesh MontageToPlay
    (:`then`
      (`KismetSystemLibrary.Delay` 0.2)
      (bind _asabp_emote (cast `/Game/Mods/_LesnovMods/EmoteMenu/ABP_Emote` (`SkeletalMeshComponent.GetAnimInstance` (`Character.Mesh` (`self.As SBZPlayer Character`))))
        (:`then`
          (bind _object (`|LoadAsset` (`|ConvertAsset` (`/Game/Mods/_LesnovMods/EmoteMenu/EmoteSettings.anim` EmoteSettings)))
            (:`then`
              (bind _asanim_sequence (cast `AnimSequence` _object))
              (`/Game/Mods/_LesnovMods/BML_Actor.AddDebugText` (`KismetSystemLibrary.GetDisplayName` _asanim_sequence)
                (:`Exec`
                  (set `/Game/Mods/_LesnovMods/EmoteMenu/ABP_Emote.Sequence` _asanim_sequence _asabp_emote))))))
        (:`CastFailed`
          (`/Game/Mods/_LesnovMods/BML_Actor.AddDebugText` "ABP_Emote Cast Failed"))))))

(event `OnTakeAnyDamage_Event_0` :!signature `self.OnTakeAnyDamage`
  (params (DamagedActor :type "Actor Object Reference") (Damage :type "Float (double-precision)") (DamageType :type "DamageType Object Reference") (InstigatedBy :type "Controller Object Reference") (DamageCauser :type "Actor Object Reference"))
  (`/Game/Mods/_LesnovMods/EmoteMenu/BP_EmoteCamera.OnEmoteCameraDisabled` (`self.EmoteCamera`)))

(event `CloseSettingMenu`
  (bind _emotesettingmenu (`self.EmoteSettingMenu`))
  (`/Engine/EditorBlueprintResources/StandardMacros.IsValid` _emotesettingmenu
    (:`Is Valid`
      (if (`Widget.IsVisible` _emotesettingmenu)
        (`/Game/Mods/_LesnovMods/BML_Actor.ToggleWidgetWithFocus` (`self.EmoteSettingMenu`) :!label _label_4
          (:`OnVisible`
            (`self.CloseEmoteMenu`))
          (:`OnNotVisible`
            (for _array_element (`/Game/Mods/_LesnovMods/EmoteMenu/Menu_EmoteSettings.Emotes` (`self.EmoteSettingMenu`))
              (bind _returnvalue (`/Game/Mods/_LesnovMods/EmoteMenu/UI_EmoteSetting.GetVolumeValue` _array_element))
              (`BlueprintMapLibrary.Map_Add` (`/Game/Mods/_LesnovMods/EmoteMenu/EmoteSavegame.EmoteVolumes` (`self.As Emote Savegame`)) (`/Game/Mods/_LesnovMods/EmoteMenu/UI_EmoteSetting.EmoteSettings` _array_element) _returnvalue))
            (`/Game/Mods/_LesnovMods/BML_Object.SaveToSlot(Macro)` (`self.As Emote Savegame`))
            (`/Game/Mods/_LesnovMods/EmoteMenu/Menu_EmoteSettings.OnMenuClosed` (`self.EmoteSettingMenu`))))))))

(event `Key|J`
  (params (Key :type "Key Structure"))
  (:`Pressed`
    (`/Engine/EditorBlueprintResources/StandardMacros.IsValid` (`self.EmoteSettingMenu`)
      (:`Is Valid`
        (goto _label_4))
      (:`Is Not Valid`
        (bind _returnvalue (`|CreateWidget` "/Game/Mods/_LesnovMods/EmoteMenu/Menu_EmoteSettings.Menu_EmoteSettings_C"))
        (bind _output_get (set `self.EmoteSettingMenu` _returnvalue))
        (`UserWidget.AddToViewport` _output_get 0)
        (for _array_element (`self.LoadedEmoteSettings`)
          (`KismetSystemLibrary.PrintString` (`KismetSystemLibrary.GetDisplayName` _array_element))
          (`/Game/Mods/_LesnovMods/EmoteMenu/Menu_EmoteSettings.CreateEmoteVoluteSelection` (`self.EmoteSettingMenu`) _array_element (`self.As Emote Savegame`)))))))

(fn `CreateEmoteMenu`
  (bind _returnvalue (`|CreateWidget` "/Game/Mods/_LesnovMods/EmoteMenu/Menu_EM_MainMenu.Menu_EM_MainMenu_C"))
  (bind _output_get (set `self.EmoteMenu` _returnvalue))
  (`UserWidget.AddToViewport` _output_get 9999)
  (`Widget.SetVisibility` _output_get "Collapsed"))

(fn `LoadEmoteAssets`
  (locals (Local_LoadedEmoteSettings :type "Array of /Game/Mods/_LesnovMods/EmoteMenu/EmoteSettings Object Reference") (Local_ArrayIndex :type Integer) (Local_ModuroRemain :type Integer :default 0) (Local_ActiveWidget :type "/Game/Mods/_LesnovMods/EmoteMenu/Menu_EM_EmoteWheel Object Reference"))
  (bind _local_activewidget (`local.Local_ActiveWidget`))
  (bind _output (`|GetArrayItem` (`local.Local_LoadedEmoteSettings`) (`local.Local_ArrayIndex`)))
  (set `local.Local_LoadedEmoteSettings` (select `bool` (`self.UseDebug(LoadedEmoteSettings)`) :`false` (`self.PreLoadedEmoteSettings`) :`true` (`self.PreLoadedEmoteSettings(DebugPurposeOnly)`)))
  (for (_ _array_index) (`local.Local_LoadedEmoteSettings`)
    (set `local.Local_ArrayIndex` _array_index)
    (bind _output_get (set `local.Local_ModuroRemain` (mod _array_index 8)))
    (if (== (`local.Local_ModuroRemain`) 0)
      (bind _returnvalue (`|CreateWidget` "/Game/Mods/_LesnovMods/EmoteMenu/Menu_EM_EmoteWheel.Menu_EM_EmoteWheel_C"))
      (`PanelWidget.AddChild` (`/Game/Mods/_LesnovMods/EmoteMenu/Menu_EM_MainMenu.WidgetSwitcher_51` (`self.EmoteMenu`)) _returnvalue)
      (bind _output_get_2 (set `local.Local_ActiveWidget` _returnvalue))
      (`self.CustomEvent_0` _output_get_2)
      (else
        (`KismetSystemLibrary.PrintString` (`KismetStringLibrary.Conv_IntToString` _output_get))))
    (`/Engine/EditorBlueprintResources/StandardMacros.IsValid` _output
      (:`Is Valid`
        (`/Game/Mods/_LesnovMods/EmoteMenu/UI_EM_Emote.UpdateDataAsset` (`|GetArrayItem` (`|MakeArray` (`/Game/Mods/_LesnovMods/EmoteMenu/Menu_EM_EmoteWheel.EM_Top` _local_activewidget) (`/Game/Mods/_LesnovMods/EmoteMenu/Menu_EM_EmoteWheel.EM_TopRight` _local_activewidget) (`/Game/Mods/_LesnovMods/EmoteMenu/Menu_EM_EmoteWheel.EM_Right` _local_activewidget) (`/Game/Mods/_LesnovMods/EmoteMenu/Menu_EM_EmoteWheel.EM_DownRight` _local_activewidget) (`/Game/Mods/_LesnovMods/EmoteMenu/Menu_EM_EmoteWheel.EM_Down` _local_activewidget) (`/Game/Mods/_LesnovMods/EmoteMenu/Menu_EM_EmoteWheel.EM_DownLeft` _local_activewidget) (`/Game/Mods/_LesnovMods/EmoteMenu/Menu_EM_EmoteWheel.EM_Left` _local_activewidget) (`/Game/Mods/_LesnovMods/EmoteMenu/Menu_EM_EmoteWheel.EM_TopLeft` _local_activewidget)) (`local.Local_ModuroRemain`)) _output))))
  (for _array_element (`local.Local_LoadedEmoteSettings`)
    (`KismetArrayLibrary.Array_AddUnique` (`self.LoadedEmoteSettings`) _array_element))
  (`WidgetSwitcher.SetActiveWidgetIndex` (`/Game/Mods/_LesnovMods/EmoteMenu/Menu_EM_MainMenu.WidgetSwitcher_51` (`self.EmoteMenu`)) 0))

(fn `NewFunction_0`
  (locals (NewLocalVar_0 :type String))
  (bind _animations (`SBZFacialAnimationCollection.Animations` (`SBZCharacter.FacialAnimationCollection` (`self.As SBZPlayer Character`))))
  (set `local.NewLocalVar_0` "Facial Data \n")
  (bind _keys (`BlueprintMapLibrary.Map_Keys` _animations))
  (for _array_element _keys
    (`/Game/Mods/_LesnovMods/BML_Object.QuickAppend` (`local.NewLocalVar_0`) (`|GetEnumeratorNameAsString` _array_element) 1)
    (for _array_element_2 (break `SBZFacialAnimationContainer` (`BlueprintMapLibrary.Map_Find` _animations _array_element))
      (`/Game/Mods/_LesnovMods/BML_Object.QuickAppend` (`local.NewLocalVar_0`) (`KismetSystemLibrary.GetDisplayName` _array_element_2) 2)))
  (`/Game/Mods/_LesnovMods/BML_Actor.AddDebugText` (`local.NewLocalVar_0`)))

(fn `PlayAnimation`
  (params (InputPin :type "SkeletalMeshComponent Object Reference") (NewAnimToPlay :type "AnimMontage Object Reference"))
  (`SkeletalMeshComponent.SetAnimationMode` InputPin "AnimationSingleNode")
  (`SkeletalMeshComponent.SetAnimation` InputPin NewAnimToPlay)
  (`SkeletalMeshComponent.PlayAnimation` InputPin NewAnimToPlay true))

(fn `PlayEmoteAnimation`
  (locals (NewLocalVar_0 :type "AnimSequence Object Reference") (Montage :type "AnimMontage Object Reference"))
  (bind _emote_settings (`self.Emote Settings`))
  (bind _emote_settings_2 (`self.Emote Settings`))
  (`self.CustomEvent_1` (`/Game/Mods/_LesnovMods/EmoteMenu/EmoteSettings.EmoteAnimation` _emote_settings) _emote_settings)
  (if (not (`/Game/Mods/_LesnovMods/EmoteMenu/EmoteSettings.IsAnimLoopable` _emote_settings_2))
    (bind _returnvalue (`AnimSequenceBase.GetPlayLength` (`/Game/Mods/_LesnovMods/EmoteMenu/EmoteSettings.EmoteAnimation` _emote_settings_2)))
    (`self.StartAnimStopTimer` _returnvalue)))

(fn `PlayMusicByEmoteSettings`
  (params (EmoteSettings :type "/Game/Mods/_LesnovMods/EmoteMenu/EmoteSettings Object Reference"))
  (bind _audio (`self.Audio`))
  (bind _audio_2 (`self.Audio`))
  (bind _emotemusic (`/Game/Mods/_LesnovMods/EmoteMenu/EmoteSettings.EmoteMusic` EmoteSettings))
  (bind (_value _returnvalue) (`BlueprintMapLibrary.Map_Find` (`/Game/Mods/_LesnovMods/EmoteMenu/EmoteSavegame.EmoteVolumes` (`self.As Emote Savegame`)) (`local.EmoteSettings`)))
  (`/Engine/EditorBlueprintResources/StandardMacros.IsValid` _emotemusic
    (:`Is Valid`
      (`AudioComponent.SetSound` _audio _emotemusic)
      (`AudioComponent.SetVolumeMultiplier` _audio (`KismetMathLibrary.SelectFloat` _value 1.0 _returnvalue))
      (`AudioComponent.Play` _audio 0.0))
    (:`Is Not Valid`
      (if (`AudioComponent.IsPlaying` _audio_2)
        (`AudioComponent.FadeOut` _audio_2 1.0 0.0 "Linear")))))

(fn `RevertAmimation`
  (`/Game/Mods/_LesnovMods/BML_Actor.IsInEditor`
    (:`InEditor`
      (bind _asfirst_person_character (cast `/Game/_InEditorTesting/FirstPersonBP/Blueprints/FirstPersonCharacter` (`GameplayStatics.GetPlayerCharacter` 0)))
      (`SkeletalMeshComponent.SetAnimationMode` (`/Game/_InEditorTesting/FirstPersonBP/Blueprints/FirstPersonCharacter.Mesh2P` _asfirst_person_character) "AnimationBlueprint"))
    (:`InGame`
      (`SkeletalMeshComponent.SetAnimationMode` (`Character.Mesh` (`self.As SBZPlayer Character`)) "AnimationBlueprint"))))

(fn `StopMusic`
  (bind _audio (`self.Audio`))
  (if (`AudioComponent.IsPlaying` _audio)
    (`AudioComponent.FadeOut` _audio 1.0 0.0 "Linear")))

(fn `ToggleEmoteMenuVisibillity`
  (params (IsVisible :type Boolean))
  (`Widget.SetVisibility` (`self.EmoteMenu`) (select `bool` IsVisible :`false` "Collapsed" :`true` "SelfHitTestInvisible" :!type "ESlateVisibility Enum")))

(fn `ToggleVisibillity(FPWeapon)`
  (params (bNewHidden :type Boolean))
  (`/Game/Mods/_LesnovMods/BML_Actor.IsInEditor`
    (:`InEditor`
      (bind _asfirst_person_character (cast `/Game/_InEditorTesting/FirstPersonBP/Blueprints/FirstPersonCharacter` (`self.As SBZPlayer Character`)))
      (`SceneComponent.SetHiddenInGame` (`/Game/_InEditorTesting/FirstPersonBP/Blueprints/FirstPersonCharacter.FP_Gun` _asfirst_person_character) (`local.bNewHidden`) false))
    (:`InGame`
      (`self.SetActorHiddenInGame` (`SBZFirstPersonCameraAttachment.EquippedWeapon` (`SBZPlayerCharacter.FPCameraAttachment` (`self.As SBZPlayer Character`))) (`local.bNewHidden`)))))

(fn `UserConstructionScript`
  (if (`self.PakageDebug`)
    ;[1 1 1] Comment
    (set `self.UseDebug(LoadedEmoteSettings)` true)
    (else
      ;[1 1 1] Comment
      (set `self.UseDebug(LoadedEmoteSettings)` (not (`KismetSystemLibrary.IsPackagedForDistribution`)))))
  (if (`self.UseDebug(LoadedEmoteSettings)`)
    (for _ (range 23)
      (`KismetArrayLibrary.Array_Add` (`self.PreLoadedEmoteSettings(DebugPurposeOnly)`) (`KismetArrayLibrary.Array_Random` (`|MakeArray` "/Game/Mods/_LesnovMods/EmoteMenu/EmoteAssets/Nested/ES_Testing03.ES_Testing03" "/Game/Mods/_LesnovMods/EmoteMenu/EmoteAssets/ES_Testing01.ES_Testing01" "/Game/Mods/_LesnovMods/EmoteMenu/EmoteAssets/ES_Testing02.ES_Testing02" :!type "/Game/Mods/_LesnovMods/EmoteMenu/EmoteSettings Object Reference"))))))