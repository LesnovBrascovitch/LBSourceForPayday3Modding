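; Skeletal-mesh prop Blueprint in the emote framework that can attach a character's mesh to a socket on the prop.
; When it receives the character mesh, and if attachment is enabled, it snaps that mesh to the socket, keeping world scale, then applies relative location and rotation offsets.
; In the editor, the construction script spawns an optional preview mesh at the same socket and offsets, set up with a preview animation.
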(event `/Game/Mods/_LesnovMods/EmoteMenu/EmoteFramework/BPI_EmoteSpawning.OnCharacterMeshReceieved`
  (params (SkeletalMeshComp :type "SkeletalMeshComponent Object Reference"))
  (if (`self.AttachCharacterMesh`)
    (`SceneComponent.K2_AttachToComponent` SkeletalMeshComp (`self.SkeletalMesh`) (`self.Socket Name`) "SnapToTarget" "SnapToTarget" "KeepWorld" true)
    (`SceneComponent.K2_SetRelativeLocationAndRotation` SkeletalMeshComp (`self.RelativeLocationOffset`) (`self.RelativeRotationOffset`) false false)))

(fn `UserConstructionScript`
  (`parent.UserConstructionScript`)
  (`/Game/Mods/_LesnovMods/BML_Actor.IsInEditor`
    (:`InEditor`
      (`/Engine/EditorBlueprintResources/StandardMacros.IsValid` (`self.PreviewMesh`)
        (:`Is Valid`
          (bind _returnvalue (`AddComponent|NODE_AddSkeletalMeshComponent-0`))
          (`SkinnedMeshComponent.SetSkinnedAssetAndUpdate` _returnvalue (`self.PreviewMesh`) true)
          (`SceneComponent.K2_AttachToComponent` _returnvalue (`self.SkeletalMesh`) (`self.Socket Name`) "KeepRelative" "KeepRelative" "KeepRelative" true)
          (`SceneComponent.K2_SetRelativeLocationAndRotation` _returnvalue (`self.RelativeLocationOffset`) (`self.RelativeRotationOffset`) false false)
          (set `SkeletalMeshComponent.AnimationData` (make `SingleAnimationPlayData` (`self.PreviewAnim`)) _returnvalue)
          (`SkeletalMeshComponent.SetAnimationMode` _returnvalue "AnimationSingleNode"))))))