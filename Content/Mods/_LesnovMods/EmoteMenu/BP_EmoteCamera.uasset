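; BP_EmoteCamera is a free-moving camera actor for the emote menu mod.
; OnControl places it behind and above the player, attaches the camera to a spring arm, takes the view target and clears player camera feedback effects.
; WASD flags and Shift speed drive a per-tick, non-swept offset along the actor's forward and right vectors.
; Space returns the view to the character, signals emote stop and disables input and tick.
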(event `self.ReceiveBeginPlay`
  (bind _sbzplayercameramanager (`/Game/Mods/_LesnovMods/BML_Actor.ValidCheck(Wait | SBZPlayerCameraManager)`)
    (:`Is Valid`
      (set `self.SBZPlayer Camera Manager` _sbzplayercameramanager))))

(event `OnControl`
  (bind _returnvalue (`GameplayStatics.GetPlayerCharacter` 0))
  (bind _player_controller (`self.Player Controller`))
  (bind _returnvalue_2 (`self.K2_GetActorLocation` _returnvalue))
  (set `self.NewVar_0` true)
  (if (not (`/Game/Mods/_LesnovMods/BML_Object.IsActiveCamera` (`self.CameraComponent`) (`self.SBZPlayer Camera Manager`)))
    (`self.K2_SetActorTransform` (`KismetMathLibrary.MakeTransform` (+ (- _returnvalue_2 (* (`self.GetActorForwardVector` _returnvalue) 250)) (* (`self.GetActorUpVector` _returnvalue) 150)) (`KismetMathLibrary.FindLookAtRotation` (`self.K2_GetActorLocation`) _returnvalue_2))))
  (`self.EnableInput` _player_controller)
  (`SceneComponent.K2_AttachToComponent` (`self.CameraComponent`) (`self.SpringArm`) "None" "SnapToTarget" "SnapToTarget" "SnapToTarget" true)
  (`PlayerController.SetViewTargetWithBlend` _player_controller self 0.0 "VTBlend_Linear" 0.0 false)
  (`self.SetActorTickEnabled` true)
  (`self.RemoveFeedbackEffects`))

(event `Key|LeftShift`
  (params (Key :type "Key Structure"))
  (:`Pressed`
    (set `self.MoveSpeed` 15.0))
  (:`Released`
    (set `self.MoveSpeed` 8.0)))

(event `OnEmoteCameraDisabled`
  (bind _player_controller (`self.Player Controller`))
  (`self.DisableInput` _player_controller)
  (`PlayerController.SetViewTargetWithBlend` _player_controller (`GameplayStatics.GetPlayerCharacter` 0) 0.0 "VTBlend_Linear" 0.0 false)
  (`self.OnEmoteStoppedKeyPressed`)
  (`self.DisableLogics`))

(event `Key|SpaceBar`
  (params (Key :type "Key Structure"))
  (:`Pressed`
    (`self.OnEmoteCameraDisabled`)))

(event `self.ReceiveTick`
  (params (DeltaSeconds :type "Float (single-precision)"))
  (`self.K2_AddActorWorldOffset` (+ (* (`self.GetActorForwardVector`) (* (+ (`KismetMathLibrary.SelectFloat` 1.0 0.0 (`self.W`)) (`KismetMathLibrary.SelectFloat` -1.0 0.0 (`self.S`))) (`self.MoveSpeed`))) (* (`self.GetActorRightVector`) (* (+ (`KismetMathLibrary.SelectFloat` 1.0 0.0 (`self.D`)) (`KismetMathLibrary.SelectFloat` -1.0 0.0 (`self.A`))) (`self.MoveSpeed`))))))

(event `Key|W` :consume false
  (params (Key :type "Key Structure"))
  (:`Pressed`
    (set `self.W` true))
  (:`Released`
    (set `self.W` false)))

(event `Key|S` :consume false
  (params (Key :type "Key Structure"))
  (:`Pressed`
    (set `self.S` true))
  (:`Released`
    (set `self.S` false)))

(event `Key|D` :consume false
  (params (Key :type "Key Structure"))
  (:`Pressed`
    (set `self.D` true))
  (:`Released`
    (set `self.D` false)))

(event `Key|A` :consume false
  (params (Key :type "Key Structure"))
  (:`Pressed`
    (set `self.A` true))
  (:`Released`
    (set `self.A` false)))

(fn `DisableLogics`
  (set `self.NewVar_0` false)
  (set `self.A` false)
  (set `self.S` false)
  (set `self.W` false)
  (set `self.D` false)
  (`self.SetActorTickEnabled` false))

(fn `UserConstructionScript`)