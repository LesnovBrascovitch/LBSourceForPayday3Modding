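; BP_HealthRemaining is an actor in the AmmoRemainingHUD mod that attaches itself to the player's first-person camera.
; BeginPlay retries each second until the SBZ character's camera attachment is valid, snaps to it, then, ten seconds later, adds Menu_AmmoRemainingHUD to the viewport, passing itself in.
; The progress-circle material setup for two planes, random Alpha timer and editor test path are all disconnected, so no health value is read here.
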(event `CustomEvent_0`
  (bind _newvar_0 (`self.NewVar_0`))
  (`/Engine/EditorBlueprintResources/StandardMacros.IsValid` _newvar_0
    (:`Is Valid`
      (`MaterialInstanceDynamic.SetScalarParameterValue` _newvar_0 "Alpha" (`KismetMathLibrary.RandomFloatInRange` 0.0 0.25)))))

(event `self.ReceiveBeginPlay`
  (`parent.ReceiveBeginPlay`)
  (bind _assbzplayer_character (`/Game/Mods/_LesnovMods/BML_Actor.ValidCheck(Wait | SBZPlayerCharacter)` :!label _label))
  (set `self.As SBZPlayer Character` _assbzplayer_character)
  (bind _output_get (set `self.FPCamera Attachment` (`SBZPlayerCharacter.FPCameraAttachment` _assbzplayer_character)))
  (`/Engine/EditorBlueprintResources/StandardMacros.IsValid` _output_get
    (:`Is Valid`
      (`self.K2_AttachToComponent` _output_get "None" "SnapToTarget" "SnapToTarget" "SnapToTarget")
      (`KismetSystemLibrary.Delay` 10.0)
      (`self.CreateDebugMenu`))
    (:`Is Not Valid`
      (`KismetSystemLibrary.Delay` 1.0)
      (goto _label))))

(fn `CreateDebugMenu`
  (bind _returnvalue (`|CreateWidget` "/Game/Mods/_LesnovMods/AmmoRemainingHUD/Menu_AmmoRemainingHUD.Menu_AmmoRemainingHUD_C" null self))
  (`UserWidget.AddToViewport` _returnvalue 999))

(fn `NewFunction_0`
  (bind _returnvalue (`KismetMaterialLibrary.CreateDynamicMaterialInstance` "/Game/UI/HUD/ProgressCircle/MI_ProgressCircle.MI_ProgressCircle"))
  (bind _output_get (set `self.NewVar_0` _returnvalue))
  (`PrimitiveComponent.SetMaterial` (`self.Plane`) 0 _output_get)
  (`PrimitiveComponent.SetMaterial` (`self.Plane1`) 0 _output_get))

(fn `UserConstructionScript`)