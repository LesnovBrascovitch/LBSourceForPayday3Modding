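; Mod actor that mutes selected hit-indicator sounds according to a DHSSavegame's per-sound flags.
; On BeginPlay it loads the save, polls until a third SBZHUDHitIndicatorWidget exists, caches the first's audio events, then clears or restores them on all.
; The O key opens a settings menu whose change event reapplies this; hiding it saves.
; Re-enabled EnemyHit receives the EnemyCriticalKilled sound instead of its own.
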(event `self.ReceiveBeginPlay`
  (`self.EnableInput` (`/Game/Mods/_LesnovMods/BML_Actor.GetLocalPlayerController(Comp)`))
  (bind _savegame (`/Game/Mods/_LesnovMods/BML_Object.HandleSaveGame` "/Game/Mods/_LesnovMods/DisableHitSound/DHSSavegame.DHSSavegame_C")
    (:`Exec`
      (bind _asdhssavegame (cast `/Game/Mods/_LesnovMods/DisableHitSound/DHSSavegame` _savegame))
      (set `self.As DHSSavegame` _asdhssavegame)
      (bind _foundwidgets (`WidgetBlueprintLibrary.GetAllWidgetsOfClass` "/Script/Starbreeze.SBZHUDHitIndicatorWidget" false :!label _label))
      (`/Engine/EditorBlueprintResources/StandardMacros.IsValid` (`|GetArrayItem` _foundwidgets 2)
        (:`Is Valid`
          (bind _output_get (set `self.Found Widgets` _foundwidgets))
          (`self.CacheSoundReference` (`|GetArrayItem` _output_get))
          (for _array_element (`self.Found Widgets`)
            (`self.RefleshAudioReference` _array_element)))
        (:`Is Not Valid`
          (`KismetSystemLibrary.Delay` 1.0)
          (goto _label))))))

(event `Key|O` :consume false
  (params (Key :type "Key Structure"))
  (:`Pressed`
    (`/Engine/EditorBlueprintResources/StandardMacros.IsValid` (`self.NewVar_0`)
      (:`Is Valid`
        (`/Game/Mods/_LesnovMods/BML_Actor.ToggleWidgetWithFocus` (`self.NewVar_0`)
          (:`OnNotVisible`
            (`/Game/Mods/_LesnovMods/BML_Object.SaveToSlot(Macro)` (`self.As DHSSavegame`)))))
      (:`Is Not Valid`
        (bind _returnvalue (`|CreateWidget` "/Game/Mods/_LesnovMods/DisableHitSound/Menu_DisableHitSoundSettings.Menu_DisableHitSoundSettings_C" null (`self.As DHSSavegame`)))
        (bind _output_get (set `self.NewVar_0` _returnvalue))
        (`UserWidget.AddToViewport` _output_get 0)
        (add `/Game/Mods/_LesnovMods/DisableHitSound/Menu_DisableHitSoundSettings.OnDisabillityChanged` _output_get (delegate `OnDisabillityChanged_Event_0`))
        (`/Game/Mods/_LesnovMods/BML_Actor.ToggleMouseCursor` true)))))

(event `OnDisabillityChanged_Event_0`
  (for _array_element (`self.Found Widgets`)
    (`self.RefleshAudioReference` _array_element)))

(fn `CacheSoundReference`
  (params (InputPin :type "SBZHUDHitIndicatorWidget Object Reference"))
  (set `self.Armor Break Audio Event` (`SBZHUDHitIndicatorWidget.ArmorBreakAudioEvent` InputPin))
  (set `self.Armor Hit Audio Event` (`SBZHUDHitIndicatorWidget.ArmorHitAudioEvent` InputPin))
  (set `self.Armor Penetration Audio Event` (`SBZHUDHitIndicatorWidget.ArmorPenetrationAudioEvent` InputPin))
  (set `self.Critical Hit Audio Event` (`SBZHUDHitIndicatorWidget.CriticalHitAudioEvent` InputPin))
  (set `self.Enemy Critical Killed Audio Event` (`SBZHUDHitIndicatorWidget.EnemyCriticalKilledAudioEvent` InputPin))
  (set `self.Enemy Hit Audio Event` (`SBZHUDHitIndicatorWidget.EnemyHitAudioEvent` InputPin))
  (set `self.Enemy Killed Audio Event` (`SBZHUDHitIndicatorWidget.EnemyKilledAudioEvent` InputPin))
  (set `self.No Damage Audio Event` (`SBZHUDHitIndicatorWidget.NoDamageAudioEvent` InputPin)))

(fn `NewFunction_0`
  (locals (NewLocalVar_0 :type String))
  (`/Game/Mods/_LesnovMods/BML_Object.QuickAppend` (`local.NewLocalVar_0`) "Old Found Widgets")
  (for _array_element (`self.Found Widgets`)
    (`/Game/Mods/_LesnovMods/BML_Object.QuickAppend` (`local.NewLocalVar_0`) (`KismetSystemLibrary.GetDisplayName` _array_element) 1))
  (`/Game/Mods/_LesnovMods/BML_Object.QuickAppend` (`local.NewLocalVar_0`) "New Found Widgets")
  (bind _foundwidgets (`WidgetBlueprintLibrary.GetAllWidgetsOfClass` "/Script/Starbreeze.SBZHUDHitIndicatorWidget" false))
  (for _array_element_2 _foundwidgets
    (`/Game/Mods/_LesnovMods/BML_Object.QuickAppend` (`local.NewLocalVar_0`) (`KismetSystemLibrary.GetDisplayName` _array_element_2) 1))
  (`/Game/Mods/_LesnovMods/BML_Actor.AddDebugText` (`local.NewLocalVar_0`)))

(fn `RefleshAudioReference`
  (params (SBZHudIndicater :type "SBZHUDHitIndicatorWidget Object Reference"))
  (bind _as_dhssavegame (`self.As DHSSavegame`))
  (`KismetSystemLibrary.PrintString` "DHS - RefleshAudioReference")
  (if (`/Game/Mods/_LesnovMods/DisableHitSound/DHSSavegame.DisableArmorBreak` _as_dhssavegame)
    (set `SBZHUDHitIndicatorWidget.ArmorBreakAudioEvent` null SBZHudIndicater)
    (else
      (set `SBZHUDHitIndicatorWidget.ArmorBreakAudioEvent` (`self.Armor Break Audio Event`) SBZHudIndicater)))
  (if (`/Game/Mods/_LesnovMods/DisableHitSound/DHSSavegame.DisableArmorHit` _as_dhssavegame)
    (set `SBZHUDHitIndicatorWidget.ArmorHitAudioEvent` null SBZHudIndicater)
    (else
      (set `SBZHUDHitIndicatorWidget.ArmorHitAudioEvent` (`self.Armor Hit Audio Event`) SBZHudIndicater)))
  (if (`/Game/Mods/_LesnovMods/DisableHitSound/DHSSavegame.DisableArmorPenetration` _as_dhssavegame)
    (set `SBZHUDHitIndicatorWidget.ArmorPenetrationAudioEvent` null SBZHudIndicater)
    (else
      (set `SBZHUDHitIndicatorWidget.ArmorPenetrationAudioEvent` (`self.Armor Penetration Audio Event`) SBZHudIndicater)))
  (if (`/Game/Mods/_LesnovMods/DisableHitSound/DHSSavegame.DisableCriticalHit` _as_dhssavegame)
    (set `SBZHUDHitIndicatorWidget.CriticalHitAudioEvent` null SBZHudIndicater)
    (else
      (set `SBZHUDHitIndicatorWidget.CriticalHitAudioEvent` (`self.Critical Hit Audio Event`) SBZHudIndicater)))
  (if (`/Game/Mods/_LesnovMods/DisableHitSound/DHSSavegame.DisableEnemyCriticalKilled` _as_dhssavegame)
    (set `SBZHUDHitIndicatorWidget.EnemyCriticalKilledAudioEvent` null SBZHudIndicater)
    (else
      (set `SBZHUDHitIndicatorWidget.EnemyCriticalKilledAudioEvent` (`self.Enemy Critical Killed Audio Event`) SBZHudIndicater)))
  (if (`/Game/Mods/_LesnovMods/DisableHitSound/DHSSavegame.DisableEnemyHit` _as_dhssavegame)
    (set `SBZHUDHitIndicatorWidget.EnemyHitAudioEvent` null SBZHudIndicater)
    (else
      (set `SBZHUDHitIndicatorWidget.EnemyHitAudioEvent` (`self.Enemy Critical Killed Audio Event`) SBZHudIndicater)))
  (if (`/Game/Mods/_LesnovMods/DisableHitSound/DHSSavegame.DisableEnemyKilled` _as_dhssavegame)
    (set `SBZHUDHitIndicatorWidget.EnemyKilledAudioEvent` null SBZHudIndicater)
    (else
      (set `SBZHUDHitIndicatorWidget.EnemyKilledAudioEvent` (`self.Enemy Killed Audio Event`) SBZHudIndicater)))
  (if (`/Game/Mods/_LesnovMods/DisableHitSound/DHSSavegame.DisableNoDamage` _as_dhssavegame)
    (set `SBZHUDHitIndicatorWidget.NoDamageAudioEvent` null SBZHudIndicater)
    (else
      (set `SBZHUDHitIndicatorWidget.NoDamageAudioEvent` (`self.No Damage Audio Event`) SBZHudIndicater))))

(fn `UserConstructionScript`)