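; Manager actor for a body-cam mod that restyles the player's view using settings from a save game.
; It applies a selectable dynamic material, chromatic aberration, saturation, vignette and exposure to the level's post-process volumes, easing the material's center with input axes.
; An optional recording overlay hides other HUD widgets, and U opens the settings menu.
; A toggleable spotlight attached to the first-person camera smoothly follows the aim.
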(event `self.ReceiveBeginPlay`
  (bind _savegame (`/Game/Mods/_LesnovMods/BML_Object.HandleSaveGame` "/Game/Mods/_LesnovMods/BodyCamPostProcess/BodyCamSavegame.BodyCamSavegame_C")
    (:`Exec`
      (bind _asbody_cam_savegame (cast `/Game/Mods/_LesnovMods/BodyCamPostProcess/BodyCamSavegame` _savegame))
      (set `self.As Body Cam Savegame` _asbody_cam_savegame)
      (bind _assbzplayer_character (`/Game/Mods/_LesnovMods/BML_Actor.ValidCheck(Wait | SBZPlayerCharacter)`))
      (set `self.As SBZPlayer Character` _assbzplayer_character)
      (bind _outactors (`GameplayStatics.GetAllActorsOfClass` "/Script/Engine.PostProcessVolume"))
      (set `self.PostProcessVolume` _outactors)
      (`self.EnableInput` (`/Game/Mods/_LesnovMods/BML_Actor.GetLocalPlayerController(Comp)`))
      (`self.OnPostProcessSelected_Event_0` (`/Game/Mods/_LesnovMods/BodyCamPostProcess/BodyCamSavegame.SelectedMaterialInterface` (`self.As Body Cam Savegame`)))
      (`self.InitializePostProcessVolume`)
      (`self.StartBodyCamText`)
      (`self.CreateBodyCamLight`))))

(event `self.ReceiveTick`
  (params (DeltaSeconds :type "Float (single-precision)"))
  (`self.UpdateBodyCamOutline` DeltaSeconds)
  (`self.UpdateBodyCamLightPosition` DeltaSeconds))

(event `CustomEvent`
  (if (`self.NewVar_0`)
    (for _array_element (`self.NewVar_1`)
      (`Widget.SetRenderOpacity` _array_element 1.0)
      (`Widget.SetVisibility` _array_element "SelfHitTestInvisible"))
    (bind _foundwidgets (`WidgetBlueprintLibrary.GetAllWidgetsOfClass` "/Game/UI/Widgets/StateMachine/WBP_UI_SM_ActionPhase.WBP_UI_SM_ActionPhase_C"))
    (for _array_element_2 _foundwidgets
      (bind _widget_pausemenu (`/Game/UI/Widgets/StateMachine/WBP_UI_SM_ActionPhase.Widget_PauseMenu` _array_element_2))
      (for _array_element_3 (`PanelWidget.GetAllChildren` (`Widget.GetParent` _widget_pausemenu))
        (if (!= _widget_pausemenu _array_element_3)
          (`Widget.SetRenderOpacity` _array_element_3 1.0)
          (`Widget.SetVisibility` _array_element_3 "SelfHitTestInvisible"))))))

(event `StartBodyCamText`
  (if (`/Game/Mods/_LesnovMods/BodyCamPostProcess/BodyCamSavegame.UseBodyCamText` (`self.As Body Cam Savegame`))
    (`/Engine/EditorBlueprintResources/StandardMacros.IsValid` (`self.MenuBodyCam`)
      (:`Is Valid`
        _)
      (:`Is Not Valid`
        (bind _returnvalue (`|CreateWidget` "/Game/Mods/_LesnovMods/BodyCamPostProcess/Menu_BodyCam_Record.Menu_BodyCam_Record_C"))
        (`UserWidget.AddToViewport` _returnvalue 0)
        (set `self.MenuBodyCam` _returnvalue)))
    (bind _foundwidgets (`WidgetBlueprintLibrary.GetAllWidgetsOfClass` "/Game/UI/Widgets/StateMachine/WBP_UI_SM_ActionPhase.WBP_UI_SM_ActionPhase_C" :!label _label))
    (`/Engine/EditorBlueprintResources/StandardMacros.IsValid` (`|GetArrayItem` _foundwidgets)
      (:`Is Valid`
        (`self.HideWidgets`))
      (:`Is Not Valid`
        (`KismetSystemLibrary.Delay` 1.0)
        (goto _label)))
    (else
      (`self.CustomEvent`))))

(event `HideWidgets`
  (set `self.NewVar_0` true)
  (bind _outactors (`/Game/Mods/_LesnovMods/BML_Actor.IsHealthBarInstalled`)
    (:`then`
      (`self.K2_DestroyActor` _outactors))
    (:`false`
      _))
  (bind _outactors_2 (`/Game/Mods/_LesnovMods/BML_Actor.IsDamagePopupInstalled`)
    (:`then`
      (`self.K2_DestroyActor` _outactors_2))
    (:`false`
      _))
  (bind _output (`/Game/Mods/_LesnovMods/BML_Actor.IsEmoteInstalled`)
    (:`then`
      (`BlueprintSetLibrary.Set_Add` (`self.IgnoreList(HideWidgets)`) (`/Game/Mods/_LesnovMods/EmoteMenu/BP_EmoteMenu.EmoteMenu` _output)))
    (:`false`
      _))
  (`BlueprintSetLibrary.Set_AddItems` (`self.IgnoreList(HideWidgets)`) (`|MakeArray` (`self.MenuBodyCam`) (`self.BodyCamSettingMenu`) :!type "UserWidget Object Reference"))
  (bind _foundwidgets (`WidgetBlueprintLibrary.GetAllWidgetsOfClass` "/Script/UMG.UserWidget"))
  (for _array_element _foundwidgets
    (if (!= (`GameplayStatics.GetObjectClass` _array_element) "/Game/UI/Widgets/StateMachine/WBP_UI_SM_ActionPhase.WBP_UI_SM_ActionPhase_C")
      (if (`BlueprintSetLibrary.Set_Contains` (`self.IgnoreList(HideWidgets)`) _array_element)
        _
        (elif (`Widget.IsVisible` _array_element)
          (`Widget.SetRenderOpacity` _array_element 0.0)
          (`Widget.SetVisibility` _array_element "Collapsed")
          (`KismetArrayLibrary.Array_AddUnique` (`self.NewVar_1`) _array_element)))))
  (bind _foundwidgets_2 (`WidgetBlueprintLibrary.GetAllWidgetsOfClass` "/Game/UI/Widgets/StateMachine/WBP_UI_SM_ActionPhase.WBP_UI_SM_ActionPhase_C"))
  (for _array_element_2 _foundwidgets_2
    (bind _widget_pausemenu (`/Game/UI/Widgets/StateMachine/WBP_UI_SM_ActionPhase.Widget_PauseMenu` _array_element_2))
    (for _array_element_3 (`PanelWidget.GetAllChildren` (`Widget.GetParent` _widget_pausemenu))
      (if (!= _widget_pausemenu _array_element_3)
        (`Widget.SetRenderOpacity` _array_element_3 0.0)
        (`Widget.SetVisibility` _array_element_3 "Collapsed"))))
  (bind _result (`BlueprintSetLibrary.Set_ToArray` (`self.IgnoreList(HideWidgets)`)))
  (for _array_element_4 _result
    (`KismetSystemLibrary.PrintString` (`KismetSystemLibrary.GetDisplayName` _array_element_4) true true (struct :`R` 1.0 :`G` 0.89111 :`A` 1.0) 15.0)))

(event `Key|U` :consume false
  (params (Key :type "Key Structure"))
  (bind _bodycamsettingmenu (`self.BodyCamSettingMenu`))
  (:`Pressed`
    (`/Engine/EditorBlueprintResources/StandardMacros.IsValid` _bodycamsettingmenu
      (:`Is Valid`
        (`/Game/Mods/_LesnovMods/BML_Actor.ToggleWidgetWithFocus` _bodycamsettingmenu
          (:`OnNotVisible`
            (`/Game/Mods/_LesnovMods/BML_Object.SaveToSlot(Macro)` (`self.As Body Cam Savegame`)))))
      (:`Is Not Valid`
        (bind _returnvalue (`|CreateWidget` "/Game/Mods/_LesnovMods/BodyCamPostProcess/Menu_BodyCamSettings.Menu_BodyCamSettings_C" null (`self.As Body Cam Savegame`) (`|GetArrayItem` (`self.PostProcessVolume`)) self))
        (bind _output_get (set `self.BodyCamSettingMenu` _returnvalue))
        (`UserWidget.AddToViewport` _output_get 0)
        (`/Game/Mods/_LesnovMods/BML_Actor.ToggleMouseCursor` true)
        (add `/Game/Mods/_LesnovMods/BodyCamPostProcess/Menu_BodyCamSettings.OnPostProcessSelected` (`self.BodyCamSettingMenu`) (`|CreateDelegate` :!event `OnPostProcessSelected_Event_0`))))))

(event `OnPostProcessSelected_Event_0`
  (params (`Material Interface` :type "MaterialInterface Object Reference"))
  (bind _output_get (set `/Game/Mods/_LesnovMods/BodyCamPostProcess/BodyCamSavegame.SelectedMaterialInterface` `Material Interface` (`self.As Body Cam Savegame`)))
  (bind _returnvalue (`KismetMaterialLibrary.CreateDynamicMaterialInstance` _output_get))
  (`self.AssignDMI` _returnvalue)
  (`self.InitializeMaterial`))

(event `InputAction|ToggleBodyCamLight`
  (params (Key :type "Key Structure"))
  (bind _bodycamlight (`self.BodyCamLight`))
  (:`Pressed`
    (`/Engine/EditorBlueprintResources/StandardMacros.IsValid` _bodycamlight
      (:`Is Valid`
        (`self.SetActorHiddenInGame` _bodycamlight (not (`Actor.bHidden` _bodycamlight)))
        (bind _sfxvolume (`/Game/Mods/_LesnovMods/BML_Object.GetSFXVolume`))
        (`GameplayStatics.PlaySound2D` "/Game/Mods/_LesnovMods/BodyCamPostProcess/SwitchLight.SwitchLight" _sfxvolume 1.0 0.0 null null)))))

(fn `AssignDMI`
  (params (DMI :type "MaterialInstanceDynamic Object Reference"))
  (set `self.DMI` DMI)
  (for _array_element (`self.PostProcessVolume`)
    (setmembers `PostProcessSettings` :`StructRef` (`PostProcessVolume.Settings` _array_element) :`WeightedBlendables` (make `WeightedBlendables` (`|MakeArray` (make `WeightedBlendable` 1.0 DMI) :!type "WeightedBlendable Structure")))))

(fn `CreateBodyCamLight`
  (bind _returnvalue (`|SpawnActorFromClass` "/Game/Mods/_LesnovMods/BodyCamPostProcess/BP_BodyCamLight.BP_BodyCamLight_C" (`KismetMathLibrary.MakeTransform` (0.0 0.0 0.0)) "AlwaysSpawn" "OverrideRootScale" null null))
  (bind _output_get (set `self.BodyCamLight` _returnvalue))
  (`self.K2_AttachToComponent` _output_get (`SBZPlayerCharacter.FPCameraAttachment` (`self.As SBZPlayer Character`)) "None" "SnapToTarget" "KeepWorld" "KeepWorld" true)
  (`self.InititializeBodyCamLight`)
  (`self.SetActorHiddenInGame` (`self.BodyCamLight`) true))

(fn `InitializeMaterial`
  (`self.SetScalarPameter` "EnableLineEffect" (`/Game/Mods/_LesnovMods/BodyCamPostProcess/BodyCamSavegame.LineEffect` (`self.As Body Cam Savegame`))))

(fn `InitializePostProcessVolume`
  (bind _as_body_cam_savegame (`self.As Body Cam Savegame`))
  (`self.SetChromaticIntensity` (`/Game/Mods/_LesnovMods/BodyCamPostProcess/BodyCamSavegame.ChromaticIntensity` _as_body_cam_savegame))
  (`self.SetSatuation` (`/Game/Mods/_LesnovMods/BodyCamPostProcess/BodyCamSavegame.SartuationIntensity` _as_body_cam_savegame))
  (`self.SetVignetteIntensity` (`/Game/Mods/_LesnovMods/BodyCamPostProcess/BodyCamSavegame.VignetteIntensity` _as_body_cam_savegame))
  (`self.SetBrightnessIntensity` (`/Game/Mods/_LesnovMods/BodyCamPostProcess/BodyCamSavegame.ExposureCompensation` _as_body_cam_savegame)))

(fn `InititializeBodyCamLight`
  (bind _as_body_cam_savegame (`self.As Body Cam Savegame`))
  (`self.SetPos(BodyCamLight)` (`/Game/Mods/_LesnovMods/BodyCamPostProcess/BodyCamSavegame.BodyCamLightPosOffset` _as_body_cam_savegame))
  (`self.SetIntensity(BodyCamLight)` (`/Game/Mods/_LesnovMods/BodyCamPostProcess/BodyCamSavegame.BodyCamLightIntensity` _as_body_cam_savegame))
  (`self.SetAttenuation(BodyCamLight)` (`/Game/Mods/_LesnovMods/BodyCamPostProcess/BodyCamSavegame.BodyCamLightAttenuation` _as_body_cam_savegame))
  (`self.SetInnerRadius(BodyCamLight)` (`/Game/Mods/_LesnovMods/BodyCamPostProcess/BodyCamSavegame.BodyCamLightInnerConeRadius` _as_body_cam_savegame))
  (`self.SetOuterRadius(BodyCamLight)` (`/Game/Mods/_LesnovMods/BodyCamPostProcess/BodyCamSavegame.BodyCamLightOuterConeRadius` _as_body_cam_savegame)))

(fn `SetAttenuation(BodyCamLight)`
  (params (NewRadius :type "Float (double-precision)"))
  (bind _bodycamlight (`self.BodyCamLight`))
  (`/Engine/EditorBlueprintResources/StandardMacros.IsValid` _bodycamlight
    (:`Is Valid`
      (`LocalLightComponent.SetAttenuationRadius` (`/Game/Mods/_LesnovMods/BodyCamPostProcess/BP_BodyCamLight.SpotLight` _bodycamlight) NewRadius))))

(fn `SetBrightnessIntensity`
  (params (Intensity :type "Float (double-precision)"))
  (for _array_element (`self.PostProcessVolume`)
    (setmembers `PostProcessSettings` :`StructRef` (`PostProcessVolume.Settings` _array_element) :`AutoExposureBias` Intensity)))

(fn `SetChromaticIntensity`
  (params (Intensity :type "Float (double-precision)"))
  (for _array_element (`self.PostProcessVolume`)
    (setmembers `PostProcessSettings` :`StructRef` (`PostProcessVolume.Settings` _array_element) :`SceneFringeIntensity` Intensity :`ChromaticAberrationStartOffset` 0.0)))

(fn `SetInnerRadius(BodyCamLight)`
  (params (NewInnerConeAngle :type "Float (double-precision)"))
  (bind _bodycamlight (`self.BodyCamLight`))
  (`/Engine/EditorBlueprintResources/StandardMacros.IsValid` _bodycamlight
    (:`Is Valid`
      (`SpotLightComponent.SetInnerConeAngle` (`/Game/Mods/_LesnovMods/BodyCamPostProcess/BP_BodyCamLight.SpotLight` _bodycamlight) NewInnerConeAngle))))

(fn `SetIntensity(BodyCamLight)`
  (params (NewIntensity :type "Float (double-precision)"))
  (bind _bodycamlight (`self.BodyCamLight`))
  (`/Engine/EditorBlueprintResources/StandardMacros.IsValid` _bodycamlight
    (:`Is Valid`
      (`LightComponent.SetIntensity` (`/Game/Mods/_LesnovMods/BodyCamPostProcess/BP_BodyCamLight.SpotLight` _bodycamlight) NewIntensity))))

(fn `SetOuterRadius(BodyCamLight)`
  (params (NewOuterConeAngle :type "Float (double-precision)"))
  (bind _bodycamlight (`self.BodyCamLight`))
  (`/Engine/EditorBlueprintResources/StandardMacros.IsValid` _bodycamlight
    (:`Is Valid`
      (`SpotLightComponent.SetOuterConeAngle` (`/Game/Mods/_LesnovMods/BodyCamPostProcess/BP_BodyCamLight.SpotLight` _bodycamlight) NewOuterConeAngle))))

(fn `SetPos(BodyCamLight)`
  (params (NewRelativeLocation :type "Vector Structure"))
  (bind _bodycamlight (`self.BodyCamLight`))
  (bind _fpcameraattachment (`SBZPlayerCharacter.FPCameraAttachment` (`self.As SBZPlayer Character`)))
  (`/Engine/EditorBlueprintResources/StandardMacros.IsValid` _bodycamlight
    (:`Is Valid`
      (`self.K2_SetActorRelativeLocation` _bodycamlight NewRelativeLocation false false)
      (`self.K2_SetActorRotation` (`self.BodyCamLight`) (`KismetMathLibrary.FindLookAtRotation` (`self.K2_GetActorLocation` (`self.BodyCamLight`)) (+ (`SceneComponent.K2_GetComponentLocation` _fpcameraattachment) (* (`SceneComponent.GetForwardVector` _fpcameraattachment) 500))) false))))

(fn `SetSatuation`
  (params (Intensity :type "Float (double-precision)"))
  (for _array_element (`self.PostProcessVolume`)
    (setmembers `PostProcessSettings` :`StructRef` (`PostProcessVolume.Settings` _array_element) :`ColorSaturation` (`KismetMathLibrary.MakeVector4` Intensity Intensity Intensity 1.0))))

(fn `SetScalarPameter`
  (params (ParameterName :type Name) (Value :type "Float (double-precision)"))
  (bind _dmi (`self.DMI`))
  (`/Engine/EditorBlueprintResources/StandardMacros.IsValid` _dmi
    (:`Is Valid`
      (`MaterialInstanceDynamic.SetScalarParameterValue` _dmi ParameterName Value))))

(fn `SetVignetteIntensity`
  (params (Intensity :type "Float (double-precision)"))
  (for _array_element (`self.PostProcessVolume`)
    (setmembers `PostProcessSettings` :`StructRef` (`PostProcessVolume.Settings` _array_element) :`VignetteIntensity` Intensity)))

(fn `UpdateBodyCamLightPosition`
  (params (DeltaSeconds :type "Float (double-precision)"))
  (bind _bodycamlight (`self.BodyCamLight`))
  (bind _fpcameraattachment (`SBZPlayerCharacter.FPCameraAttachment` (`self.As SBZPlayer Character`)))
  (bind _returnvalue (`KismetMathLibrary.RInterpTo` (`self.CurrentRotation(BodyCamLight)`) (`KismetMathLibrary.FindLookAtRotation` (`self.K2_GetActorLocation` _bodycamlight) (+ (`SceneComponent.K2_GetComponentLocation` _fpcameraattachment) (* (`SceneComponent.GetForwardVector` _fpcameraattachment) 1500))) DeltaSeconds 33.0))
  (`/Engine/EditorBlueprintResources/StandardMacros.IsValid` _bodycamlight
    (:`Is Valid`
      (`self.K2_SetActorRotation` _bodycamlight _returnvalue false)
      (set `self.CurrentRotation(BodyCamLight)` _returnvalue))))

(fn `UpdateBodyCamOutline`
  (params (DeltaSeconds :type "Float (double-precision)"))
  (bind _dmi (`self.DMI`))
  (bind _returnvalue (`KismetSystemLibrary.MakeLiteralDouble` (`self.OutShadownOffsetMax`)))
  (bind _returnvalue_2 (`KismetSystemLibrary.MakeLiteralDouble` (`self.OutShadownOffsetMin`)))
  (`/Engine/EditorBlueprintResources/StandardMacros.IsValid` _dmi
    (:`Is Valid`
      (bind _output_get (set `self.CurrentLocation` (`KismetMathLibrary.VInterpTo_Constant` (`self.CurrentLocation`) (`KismetMathLibrary.MakeVector` (+ (`KismetMathLibrary.FClamp` (`self.GetInputAxisKeyValue`) _returnvalue_2 _returnvalue) 0.5) (+ (`KismetMathLibrary.FClamp` (`self.GetInputAxisKeyValue`) _returnvalue_2 _returnvalue) 0.5)) DeltaSeconds 0.1)))
      (`MaterialInstanceDynamic.SetVectorParameterValue` _dmi "CenterPosition (V2)" (`KismetMathLibrary.Conv_VectorToLinearColor` _output_get)))))

(fn `UserConstructionScript`
  (bind _returnvalue (`KismetMathLibrary.Abs` (`self.OutShadownOffset`)))
  (set `self.OutShadownOffsetMax` _returnvalue)
  (set `self.OutShadownOffsetMin` (* -1 _returnvalue)))