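; Bodycam mod actor that applies fisheye post-process materials to every PostProcessVolume, adds a bodycam overlay and hides the HUD.
; A flag selects either a lens settings menu with material toggle, input-driven lens-centre drift and muted hit-indicator audio, or a fixed lens with chromatic aberration and timed UI re-hiding.
; Hotkeys swap, invert or clear the lens, mute hit audio and destroy AI crew.
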(event `self.ReceiveBeginPlay`
  (bind _newvar_0 (`self.NewVar_0`))
  (bind _savegame (`/Game/Mods/_LesnovMods/BML_Object.HandleSaveGame` "/Game/Mods/_LesnovMods/BodyCamPostProcess/BodyCamSavegame.BodyCamSavegame_C")
    (:`Exec`
      (bind _asbody_cam_savegame (cast `/Game/Mods/_LesnovMods/BodyCamPostProcess/BodyCamSavegame` _savegame))
      (set `self.As Body Cam Savegame` _asbody_cam_savegame)
      (bind _assbzplayer_character (`/Game/Mods/_LesnovMods/BML_Actor.ValidCheck(Wait | SBZPlayerCharacter)`))
      (set `self.As SBZPlayer Character` _assbzplayer_character)
      (bind _outactors (`GameplayStatics.GetAllActorsOfClass` "/Script/Engine.PostProcessVolume"))
      (set `self.Out Actors` _outactors)
      (`self.EnableInput` (`/Game/Mods/_LesnovMods/BML_Actor.GetLocalPlayerController(Comp)`))
      (bind _returnvalue (`|CreateWidget` "/Game/Mods/_LesnovMods/BodyCamPostProcess/Menu_BodyCam.Menu_BodyCam_C"))
      (`UserWidget.AddToViewport` _returnvalue 0)
      (set `self.NewVar_5` _returnvalue)
      (bind _foundwidgets (`WidgetBlueprintLibrary.GetAllWidgetsOfClass` "/Script/Starbreeze.SBZHUDWidgetBase" false))
      (for _array_element _foundwidgets
        (`Widget.SetRenderOpacity` _array_element 0.0)
        (`Widget.SetVisibility` _array_element "Hidden"))
      (if (`self.NewVar_4`)
        (bind _returnvalue_2 (`KismetMaterialLibrary.CreateDynamicMaterialInstance` "/Game/Mods/_LesnovMods/BodyCamPostProcess/MI_FishLens_02.MI_FishLens_02"))
        (set `self.NewVar_0` _returnvalue_2)
        (bind _returnvalue_3 (`KismetMaterialLibrary.CreateDynamicMaterialInstance` "/Game/Mods/_LesnovMods/BodyCamPostProcess/MI_FishLens_01.MI_FishLens_01"))
        (set `self.NewVar_1` _returnvalue_3)
        (bind _outactors_2 (`GameplayStatics.GetAllActorsOfClass` "/Script/Engine.PostProcessVolume"))
        (set `self.Out Actors` _outactors_2)
        (`self.AssignDMI` (`self.NewVar_1`))
        (bind _returnvalue_4 (`|CreateWidget` "/Game/Mods/_LesnovMods/BodyCamPostProcess/Menu_FishLensSettings.Menu_FishLensSettings_C"))
        (bind _output_get (set `self.NewVar_2` _returnvalue_4))
        (`/Game/Mods/_LesnovMods/BodyCamPostProcess/Menu_FishLensSettings.CustomEvent_0` _output_get (`self.NewVar_0`) (`self.Out Actors`))
        (`UserWidget.AddToViewport` _returnvalue_4 0)
        (add `Button.OnClicked` (`/Game/Mods/_LesnovMods/BodyCamPostProcess/Menu_FishLensSettings.Button_0` _returnvalue_4) (delegate `OnClicked_Event_0`))
        (`/Game/Mods/_LesnovMods/BodyCamPostProcess/Menu_FishLensSettings.CustomEvent_0` (`self.NewVar_2`) _newvar_0 (`self.Out Actors`))
        (`self.AssignDMI` _newvar_0)
        (bind _foundwidgets_2 (`WidgetBlueprintLibrary.GetAllWidgetsOfClass` "/Script/Starbreeze.SBZHUDHitIndicatorWidget" false :!label _label))
        (`/Engine/EditorBlueprintResources/StandardMacros.IsValid` (`|GetArrayItem` _foundwidgets_2)
          (:`Is Valid`
            (for _array_element_2 _foundwidgets_2
              (set `SBZHUDHitIndicatorWidget.EnemyHitAudioEvent` null _array_element_2)
              (set `SBZHUDHitIndicatorWidget.EnemyKilledAudioEvent` null _array_element_2)
              (set `SBZHUDHitIndicatorWidget.CriticalHitAudioEvent` null _array_element_2)
              (set `SBZHUDHitIndicatorWidget.ArmorBreakAudioEvent` null _array_element_2)
              (set `SBZHUDHitIndicatorWidget.ArmorHitAudioEvent` null _array_element_2)
              (set `SBZHUDHitIndicatorWidget.ArmorPenetrationAudioEvent` null _array_element_2)
              (set `SBZHUDHitIndicatorWidget.NoDamageAudioEvent` null _array_element_2)))
          (:`Is Not Valid`
            (`KismetSystemLibrary.Delay` 1.0)
            (goto _label)))
        (else
          (bind _returnvalue_5 (`KismetMaterialLibrary.CreateDynamicMaterialInstance` "/Game/Mods/_LesnovMods/BodyCamPostProcess/MI_FishLens_02.MI_FishLens_02"))
          (`self.AssignDMI` _returnvalue_5)
          (`self.SetChromaticIntensity` 1.3)
          (`KismetSystemLibrary.K2_SetTimerDelegate` (delegate `CustomEvent_0`) 5.0 true)
          (bind _foundwidgets_3 (`WidgetBlueprintLibrary.GetAllWidgetsOfClass` "/Script/UMG.UserWidget" :!label _label_2))
          (for _array_element_3 _foundwidgets_3
            (if (not (`BlueprintSetLibrary.Set_Contains` (`|MakeSet` (`self.NewVar_5`) (`self.BodyCamSettingMenu`) :!type "UserWidget Object Reference") _array_element_3))
              (`Widget.SetRenderOpacity` _array_element_3 0.0)
              (`Widget.SetVisibility` _array_element_3 "Hidden")
              (`KismetSystemLibrary.K2_SetTimerDelegate` (delegate `CustomEvent_1`) 1.0 true))))))))

(event `Key|Ctrl+H`
  (params (Key :type "Key Structure"))
  (:`Pressed`
    (bind _returnvalue (`KismetMaterialLibrary.CreateDynamicMaterialInstance` "/Game/Mods/_LesnovMods/BodyCamPostProcess/MI_FishLens_02.MI_FishLens_02"))
    (`self.AssignDMI` _returnvalue)))

(event `OnClicked_Event_0`
  (bind _newvar_1 (`self.NewVar_1`))
  (bind _newvar_0 (`self.NewVar_0`))
  (bind _out_actors (`self.Out Actors`))
  (`/Engine/EditorBlueprintResources/StandardMacros.FlipFlop`
    (:`A`
      (`/Game/Mods/_LesnovMods/BodyCamPostProcess/Menu_FishLensSettings.CustomEvent_0` (`self.NewVar_2`) _newvar_1 _out_actors)
      (`self.AssignDMI` _newvar_1))
    (:`B`
      (`/Game/Mods/_LesnovMods/BodyCamPostProcess/Menu_FishLensSettings.CustomEvent_0` (`self.NewVar_2`) _newvar_0 _out_actors)
      (`self.AssignDMI` _newvar_0))))

(event `Key|H`
  (params (Key :type "Key Structure"))
  (:`Pressed`
    (bind _returnvalue (`KismetMaterialLibrary.CreateDynamicMaterialInstance` "/Game/Mods/_LesnovMods/BodyCamPostProcess/MI_FishLens_02_Invert.MI_FishLens_02_Invert"))
    (`self.AssignDMI` _returnvalue)))

(event `Key|Alt+H`
  (params (Key :type "Key Structure"))
  (:`Pressed`
    (`self.AssignDMI` null)))

(event `self.ReceiveTick`
  (params (DeltaSeconds :type "Float (single-precision)"))
  (bind _newvar_0 (`self.NewVar_0`))
  (`/Engine/EditorBlueprintResources/StandardMacros.IsValid` _newvar_0
    (:`Is Valid`
      (bind _output_get (set `self.NewVar_3` (`KismetMathLibrary.VInterpTo` (`self.NewVar_3`) (`KismetMathLibrary.MakeVector` (+ (`KismetMathLibrary.FClamp` (`self.GetInputAxisKeyValue`) -0.05 0.05) 0.5) (+ (`KismetMathLibrary.FClamp` (`self.GetInputAxisKeyValue`) -0.05 0.05) 0.5)) DeltaSeconds 1.0)))
      (`MaterialInstanceDynamic.SetVectorParameterValue` _newvar_0 "CenterPosition (V2)" (`KismetMathLibrary.Conv_VectorToLinearColor` _output_get)))))

(event `CustomEvent_0`
  (goto _label_2))

(event `CustomEvent_1`
  (`/Game/Mods/_LesnovMods/BodyCamPostProcess/Menu_BodyCam.Menu_BodyCam_AutoGenFunc` (`self.NewVar_5`)))

(event `Key|LeftControl`
  (params (Key :type "Key Structure"))
  (:`Pressed`
    (bind _foundwidgets (`WidgetBlueprintLibrary.GetAllWidgetsOfClass` "/Script/Starbreeze.SBZHUDHitIndicatorWidget" false))
    (for _array_element _foundwidgets
      (set `SBZHUDHitIndicatorWidget.EnemyHitAudioEvent` null _array_element)
      (set `SBZHUDHitIndicatorWidget.EnemyKilledAudioEvent` null _array_element)
      (set `SBZHUDHitIndicatorWidget.CriticalHitAudioEvent` null _array_element)
      (set `SBZHUDHitIndicatorWidget.ArmorBreakAudioEvent` null _array_element)
      (set `SBZHUDHitIndicatorWidget.ArmorHitAudioEvent` null _array_element)
      (set `SBZHUDHitIndicatorWidget.ArmorPenetrationAudioEvent` null _array_element)
      (set `SBZHUDHitIndicatorWidget.NoDamageAudioEvent` null _array_element))))

(event `Key|B`
  (params (Key :type "Key Structure"))
  (:`Pressed`
    (bind _outactors (`GameplayStatics.GetAllActorsOfClass` "/Script/Starbreeze.SBZAICrewCharacter"))
    (`self.K2_DestroyActor` _outactors)))

(fn `AssignDMI`
  (params (DMI :type "MaterialInstanceDynamic Object Reference"))
  (for _array_element (`self.Out Actors`)
    (setmembers `PostProcessSettings` :`StructRef` (`PostProcessVolume.Settings` _array_element) :`WeightedBlendables` (make `WeightedBlendables` (`|MakeArray` (make `WeightedBlendable` 1.0 DMI) :!type "WeightedBlendable Structure")))))

(fn `SetChromaticIntensity`
  (params (Intensity :type "Float (double-precision)"))
  (for _array_element (`self.Out Actors`)
    (setmembers `PostProcessSettings` :`StructRef` (`PostProcessVolume.Settings` _array_element) :`SceneFringeIntensity` Intensity :`ChromaticAberrationStartOffset` 0.0)))

(fn `UserConstructionScript`)