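; BP_FreeCam is a test free-camera actor that enables player input and snaps its camera onto a spring arm on BeginPlay.
; WASD keys set movement flags, Tick applies GetTargetOffset as a world offset, and Left Shift disables input.
; GetTargetOffset holds forward/right vector math scaled by MoveSpeed, but that expression is left unused, so the movement appears unfinished.
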(event `self.ReceiveBeginPlay`
  (`self.EnableInput` (`self.Player Controller`))
  (`SceneComponent.K2_AttachToComponent` (`self.CameraComponent`) (`self.SpringArm`) "None" "SnapToTarget" "SnapToTarget" "SnapToTarget" true))

(event `Key|LeftShift`
  (params (Key :type "Key Structure"))
  (:`Pressed`
    (`self.DisableInput` (`self.Player Controller`))))

(event `self.ReceiveTick`
  (params (DeltaSeconds :type "Float (single-precision)"))
  (`self.K2_AddActorWorldOffset` (+ (* (`self.GetActorForwardVector`) (* (+ (`KismetMathLibrary.SelectFloat` 1.0 0.0 (`self.W`)) (`KismetMathLibrary.SelectFloat` -1.0 0.0 (`self.S`))) (`self.MoveSpeed`))) (* (`self.GetActorRightVector`) (* (+ (`KismetMathLibrary.SelectFloat` 1.0 0.0 (`self.D`)) (`KismetMathLibrary.SelectFloat` -1.0 0.0 (`self.A`))) (`self.MoveSpeed`))))))

(event `Key|W` :consume false
  (params (Key :type "Key Structure"))
  (:`Pressed`
    (set `self.W` true))
  (:`Released`
    (set `self.W` false)))

(event `Key|S` :consume false
  (params (Key :type "Key Structure"))
  (:`Pressed`
    (set `self.S` true))
  (:`Released`
    (set `self.S` false)))

(event `Key|D` :consume false
  (params (Key :type "Key Structure"))
  (:`Pressed`
    (set `self.D` true))
  (:`Released`
    (set `self.D` false)))

(event `Key|A` :consume false
  (params (Key :type "Key Structure"))
  (:`Pressed`
    (set `self.A` true))
  (:`Released`
    (set `self.A` false)))

(fn `UserConstructionScript`)