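; Debug testing-ground actor for a mod that creates an on-screen test menu and binds to the local SBZ player character.
; A looping camera line trace feeds the hit actor to the menu and snaps a preview instance to the surface, aligned to its normal.
; MakeSpawnInstance replaces that preview, and hotkeys spawn copies of it, toggle the cursor and free camera, or show hidden widgets.
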(event `CustomEvent_1`
  (`Widget.SetVisibility` (`self.MenuTestingGround`) "SelfHitTestInvisible"))

(event `self.ReceiveBeginPlay`
  (bind _playercontroller (`/Game/Mods/_LesnovMods/BML_Actor.GetLocalPlayerController(Comp)`))
  (`parent.ReceiveBeginPlay`)
  (`self.CreateDebugMenu`)
  (bind _assbzplayer_character (`/Game/Mods/_LesnovMods/BML_Actor.ValidCheck(Wait | SBZPlayerCharacter)`))
  (set `self.As SBZPlayer Character` _assbzplayer_character)
  (set `self.FPCamera Attachment` (`SBZPlayerCharacter.FPCameraAttachment` _assbzplayer_character))
  (`KismetSystemLibrary.K2_SetTimerDelegate` (`|CreateDelegate` :!event `LinetraceLogic`) 0.01 true)
  (`self.EnableInput` _playercontroller)
  (set `self.PlayerController` _playercontroller)
  (`/Game/Mods/_LesnovMods/_TestingGround/Menu/QuickTestingMenu/Menu_TG_QuickTesting.OnPlayerCharacterAssigned` (`self.MenuTestingGround`) (`self.As SBZPlayer Character`)))

(event `LinetraceLogic`
  (bind _menutestingground (`self.MenuTestingGround`))
  (bind _fpcamera_attachment (`self.FPCamera Attachment`))
  (bind _returnvalue (`SceneComponent.K2_GetComponentLocation` _fpcamera_attachment))
  (bind _ui_displaytexts (`/Game/Mods/_LesnovMods/_TestingGround/Menu/QuickTestingMenu/Menu_TG_QuickTesting.UI_DisplayTexts` (`self.MenuTestingGround`)))
  (bind (_outhit _returnvalue_2) (`KismetSystemLibrary.LineTraceSingle` _returnvalue (+ _returnvalue (* (`SceneComponent.GetForwardVector` _fpcamera_attachment) 30000)) "TraceTypeQuery2" false (`|MakeArray` (`self.As SBZPlayer Character`) (`self.InstancedActor`) :!type "Actor Object Reference")))
  (set `self.Out Hit` _outhit)
  (if _returnvalue_2
    (bind (_bblockinghit _binitialoverlap _time _distance _location _impactpoint _normal _impactnormal _physmat _hitactor) (`GameplayStatics.BreakHitResult` _outhit))
    (set `self.Location` _location)
    (bind _output_get (set `self.Hit Actor` _hitactor))
    (`/Game/Mods/_LesnovMods/_TestingGround/UI_DisplayTexts.SetText` _ui_displaytexts (`KismetTextLibrary.Conv_StringToText` (`KismetSystemLibrary.GetDisplayName` _output_get)))
    (set `/Game/Mods/_LesnovMods/_TestingGround/Menu/QuickTestingMenu/Menu_TG_QuickTesting.HitActor` _output_get _menutestingground)
    (`self.Update Instanced Spawn Target` (`self.Out Hit`))
    (else
      (set `self.Hit Actor` null)
      (`/Game/Mods/_LesnovMods/_TestingGround/UI_DisplayTexts.SetText` _ui_displaytexts "")
      (set `/Game/Mods/_LesnovMods/_TestingGround/Menu/QuickTestingMenu/Menu_TG_QuickTesting.HitActor` null _menutestingground))))

(event `Key|M` :consume false
  (params (Key :type "Key Structure"))
  ;[1 1 1] M - Toggle Mouse Cursor
  (:`Pressed`
    (`/Game/Mods/_LesnovMods/BML_Object.ToggleMouseCursor` (`self.PlayerController`))))

(event `Key|J` :consume false
  (params (Key :type "Key Structure"))
  (bind _instancedactor (`self.InstancedActor`))
  ;[1 1 1] J - Spawn Class
  (:`Pressed`
    (`/Engine/EditorBlueprintResources/StandardMacros.IsValid` _instancedactor
      (:`Is Valid`
        (`|SpawnActorFromClass` (`GameplayStatics.GetObjectClass` _instancedactor) (`self.GetTransform` _instancedactor) "AlwaysSpawn" "OverrideRootScale" null null)))))

(event `Key|Six` :consume false
  (params (Key :type "Key Structure"))
  ;[1 1 1] 6 - Toggle Free Camera
  (:`Pressed`
    (`/Game/Mods/_LesnovMods/_TestingGround/Menu/QuickTestingMenu/Menu_TG_QuickTesting.SwitchFreeCamera` (`/Game/Mods/_LesnovMods/_TestingGround/Menu/Menu_TGMain.Menu_QuickTesting` (`self.MenuMain`)))))

(event `Key|Seven` :consume false
  (params (Key :type "Key Structure"))
  (:`Pressed`
    (`/Game/Mods/_LesnovMods/_TestingGround/Menu/QuickTestingMenu/Menu_TG_QuickTesting.ShowHiddenWidgets` (`/Game/Mods/_LesnovMods/_TestingGround/Menu/Menu_TGMain.Menu_QuickTesting` (`self.MenuMain`)))))

(fn `AddText`
  (params (String :type String))
  (bind _menu_quicktesting (`/Game/Mods/_LesnovMods/_TestingGround/Menu/Menu_TGMain.Menu_QuickTesting` (`self.MenuMain`)))
  (`/Engine/EditorBlueprintResources/StandardMacros.IsValid` (`self.MenuMain`)
    (:`Is Valid`
      (`/Engine/EditorBlueprintResources/StandardMacros.IsValid` _menu_quicktesting
        (:`Is Valid`
          (`/Game/Mods/_LesnovMods/_TestingGround/Menu/QuickTestingMenu/Menu_TG_QuickTesting.AddText` _menu_quicktesting String))))))

(fn `CreateDebugMenu`
  (bind _returnvalue (`|CreateWidget` "/Game/Mods/_LesnovMods/_TestingGround/Menu/Menu_TGMain.Menu_TGMain_C"))
  (`UserWidget.AddToViewport` _returnvalue 15000)
  (set `self.MenuMain` _returnvalue)
  (bind _output_get (set `self.MenuTestingGround` (`/Game/Mods/_LesnovMods/_TestingGround/Menu/Menu_TGMain.Menu_QuickTesting` _returnvalue)))
  (`/Game/Mods/_LesnovMods/_TestingGround/Menu/QuickTestingMenu/Menu_TG_QuickTesting.AddText` _output_get "Print in editor"))

(fn `MakeSpawnInstance`
  (params (ActorClass :type "Actor Class Reference"))
  (locals (NewLocalVar_0 :type "Actor Object Reference"))
  (bind _instancedactor (`self.InstancedActor`))
  (`/Engine/EditorBlueprintResources/StandardMacros.IsValid` _instancedactor
    (:`Is Valid`
      (`self.K2_DestroyActor` _instancedactor))
    (:`Is Not Valid`
      _))
  (if (`KismetSystemLibrary.IsValidClass` ActorClass)
    (bind _returnvalue (`|SpawnActorFromClass` ActorClass (`KismetMathLibrary.MakeTransform` (0.0 0.0 0.0)) "AlwaysSpawn" "OverrideRootScale" null null))
    (set `self.InstancedActor` _returnvalue)))

(fn `NewFunction_0`
  (if (`GameplayStatics.BreakHitResult` (`self.Out Hit`))
    _))

(fn `Spawn`
  (returns (NewParam :type Boolean) (`Out Hit` :type "HitResult Structure"))
  (return false (`self.Out Hit`)))

(fn `Update Instanced Spawn Target`
  (params (Hit :type "HitResult Structure (by ref)"))
  (bind (_bblockinghit _binitialoverlap _time _distance _location _impactpoint _normal) (`GameplayStatics.BreakHitResult` Hit))
  (bind _instancedactor (`self.InstancedActor`))
  (`/Engine/EditorBlueprintResources/StandardMacros.IsValid` _instancedactor
    (:`Is Valid`
      (`self.K2_SetActorTransform` _instancedactor (`KismetMathLibrary.MakeTransform` _location (`KismetMathLibrary.MakeRotFromZ` _normal)) false false))))

(fn `UserConstructionScript`)