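; Mod Blueprint that gives the local player a left-handed first-person view and adds a dot overlay for aiming.
; On BeginPlay it gets the SBZ player character through a wait-for-valid helper and mirrors its FPCameraAttachment with a negative Y scale.
; It also adds a hidden Menu_SimpleDot widget to the viewport and enables input.
; A timeline fades the dot in while right mouse is held and reverses on release.
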(event `self.ReceiveBeginPlay`
  (bind _assbzplayer_character (`/Game/Mods/_LesnovMods/BML_Actor.ValidCheck(Wait | SBZPlayerCharacter)`))
  (bind _output_get (set `self.As SBZPlayer Character` _assbzplayer_character))
  (bind _output_get_2 (set `self.FPCamera Attachment` (`SBZPlayerCharacter.FPCameraAttachment` _output_get)))
  (`SceneComponent.SetRelativeScale3D` _output_get_2 (1.0 -1.0 1.0))
  (bind _returnvalue (`|CreateWidget` "/Game/Mods/_LesnovMods/LeftHandedStyle/Menu_SimpleDot.Menu_SimpleDot_C"))
  (`UserWidget.AddToViewport` _returnvalue 888)
  (`self.EnableInput` (`/Game/Mods/_LesnovMods/BML_Actor.GetLocalPlayerController(Comp)`))
  (bind _output_get_3 (set `self.ADSHud` _returnvalue))
  (`Widget.SetRenderOpacity` _output_get_3 0.0))

(event `Key|RightMouseButton` :consume false
  (params (Key :type "Key Structure"))
  (:`Pressed`
    (bind (_direction _newtrack_0) (`Timeline|Timeline_0` :!label _label)
      (:`Update`
        (`Widget.SetRenderOpacity` (`self.ADSHud`) (`KismetMathLibrary.Lerp` 0.0 1.0 _newtrack_0)))))
  (:`Released`
    (goto _label :!via `Reverse`)))

(fn `UserConstructionScript`)