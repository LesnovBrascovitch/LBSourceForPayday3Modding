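; Mod actor that saves per-level directional light and skylight settings and applies them when the level starts.
; On BeginPlay it loads a save game, looks up the current level name and sets intensity and color on all DirectionalLight and SkyLight actors.
; The L key toggles a lazily created menu widget with mouse cursor, whose save event stores settings under the level name, writes the slot and hides the menu.
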(event `self.ReceiveBeginPlay`
  (bind _savegame (`/Game/Mods/_LesnovMods/BML_Object.HandleSaveGame` "/Game/Mods/_LesnovMods/LevelLightsSettings/LevelLightSettingsSaveGame.LevelLightSettingsSaveGame_C")
    (:`Exec`
      (bind _aslevel_light_settings_save_game (cast `/Game/Mods/_LesnovMods/LevelLightsSettings/LevelLightSettingsSaveGame` _savegame))
      (set `self.As Level Light Settings Save Game` _aslevel_light_settings_save_game)
      (`self.EnableInput` (`/Game/Mods/_LesnovMods/BML_Actor.GetLocalPlayerController(Comp)`))
      (bind _returnvalue (`GameplayStatics.GetCurrentLevelName` true))
      (bind (_value _returnvalue_2) (`BlueprintMapLibrary.Map_Find` (`/Game/Mods/_LesnovMods/LevelLightsSettings/LevelLightSettingsSaveGame.LevelLightSettingsList` (`self.As Level Light Settings Save Game`)) _returnvalue))
      (if _returnvalue_2
        (`self.UpdateDirectionalLight` _value)
        (`self.UpdateSkyLight` _value)))))

(event `OnMenuCreated`
  (add `/Game/Mods/_LesnovMods/LevelLightsSettings/HudMenu_LevelLight.OnSaveButtonPressed` (`self.HubMenu`) (delegate `OnSaveButtonPressed_Event_0`)))

(event `OnSaveButtonPressed_Event_0`
  (params (LevelLightSettings :type "/Game/Mods/_LesnovMods/LevelLightsSettings/S_LevelLightSettings Structure"))
  (bind _as_level_light_settings_save_game (`self.As Level Light Settings Save Game`))
  (bind _returnvalue (`GameplayStatics.GetCurrentLevelName` true))
  (`BlueprintMapLibrary.Map_Add` (`/Game/Mods/_LesnovMods/LevelLightsSettings/LevelLightSettingsSaveGame.LevelLightSettingsList` _as_level_light_settings_save_game) _returnvalue LevelLightSettings)
  (`/Game/Mods/_LesnovMods/BML_Object.SaveToSlot(Macro)` _as_level_light_settings_save_game)
  (`KismetSystemLibrary.Delay` 0.2)
  (set `PlayerController.bShowMouseCursor` false (`/Game/Mods/_LesnovMods/BML_Actor.GetLocalPlayerController(Comp)`))
  (`Widget.SetVisibility` (`self.HubMenu`) "Collapsed"))

(event `OnMenuOpen`
  (`/Game/Mods/_LesnovMods/LevelLightsSettings/HudMenu_LevelLight.UpdateLevelName` (`self.HubMenu`))
  (`KismetSystemLibrary.Delay` 0.2)
  (set `PlayerController.bShowMouseCursor` true (`/Game/Mods/_LesnovMods/BML_Actor.GetLocalPlayerController(Comp)`)))

(event `Key|L` :consume false
  (params (Key :type "Key Structure"))
  (:`Pressed`
    (`self.CreateHubMenu`)))

(fn `CreateHubMenu`
  (`/Engine/EditorBlueprintResources/StandardMacros.IsValid` (`self.HubMenu`)
    (:`Is Valid`
      (if (`Widget.IsVisible` (`self.HubMenu`))
        (`Widget.SetVisibility` (`self.HubMenu`) "Collapsed")
        (set `PlayerController.bShowMouseCursor` false (`/Game/Mods/_LesnovMods/BML_Actor.GetLocalPlayerController(Comp)`))
        (else
          (`Widget.SetVisibility` (`self.HubMenu`) "SelfHitTestInvisible")
          (`self.OnMenuOpen` :!label _label))))
    (:`Is Not Valid`
      (bind _returnvalue (`|CreateWidget` "/Game/Mods/_LesnovMods/LevelLightsSettings/HudMenu_LevelLight.HudMenu_LevelLight_C" null null))
      (`UserWidget.AddToViewport` _returnvalue 9999)
      (set `self.HubMenu` _returnvalue)
      (`self.OnMenuCreated`)
      (goto _label))))

(fn `UpdateDirectionalLight`
  (params (S_LevelLightSettings :type "/Game/Mods/_LesnovMods/LevelLightsSettings/S_LevelLightSettings Structure (by ref)"))
  (bind (_membervar _directionalintensity _directionalr _directionalg _directionalb) (break `/Game/Mods/_LesnovMods/LevelLightsSettings/S_LevelLightSettings` S_LevelLightSettings))
  (bind _outactors (`GameplayStatics.GetAllActorsOfClass` "/Script/Engine.DirectionalLight"))
  (for _array_element _outactors
    (bind _lightcomponent (`Light.LightComponent` _array_element))
    (`LightComponent.SetIntensity` _lightcomponent _directionalintensity)
    (`LightComponent.SetIntensity` _lightcomponent _directionalintensity)
    (`LightComponent.SetLightColor` _lightcomponent (make `LinearColor` _directionalr _directionalg _directionalb 1.0) true)))

(fn `UpdateSkyLight`
  (params (S_LevelLightSettings :type "/Game/Mods/_LesnovMods/LevelLightsSettings/S_LevelLightSettings Structure (by ref)"))
  (bind (_membervar _directionalintensity _directionalr _directionalg _directionalb _skylightintensity _skylightr _skylightg _skylightb) (break `/Game/Mods/_LesnovMods/LevelLightsSettings/S_LevelLightSettings` S_LevelLightSettings))
  (bind _outactors (`GameplayStatics.GetAllActorsOfClass` "/Script/Engine.SkyLight"))
  (for _array_element _outactors
    (bind _lightcomponent (`SkyLight.LightComponent` _array_element))
    (`SkyLightComponent.SetIntensity` _lightcomponent _skylightintensity)
    (`SkyLightComponent.SetLightColor` _lightcomponent (make `LinearColor` _skylightr _skylightg _skylightb 1.0))))

(fn `UserConstructionScript`)