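; Kill counter mod actor that shows a HUD of kills and damage per player.
; Game event broker damage events feed widget rows keyed by PlayerState, with a 15-second timer adding rows for new players.
; K toggles a settings menu for layout and visibility, persisted in a save game.
; A timeline slides the HUD aside when all players reach escape, and an editor-only path fakes kills and damage for testing.
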(event `OnPlayerKill`
  (params (SBZPlayerCharacter :type "SBZPlayerCharacter Object Reference"))
  (bind (_value _returnvalue) (`BlueprintMapLibrary.Map_Find` (`self.As SBZPlayer Character_0`) (`Pawn.PlayerState` SBZPlayerCharacter)))
  ;[1 1 1] OnPlayerKill
  (if _returnvalue
    (`/Game/Mods/_LesnovMods/KillCounter/UI_KillCount.OnPlayerKills` _value)))

(event `OnPlayerDealDamage`
  (params (SBZPlayerCharacter :type "SBZPlayerCharacter Object Reference") (Damage :type Integer))
  (bind (_value _returnvalue) (`BlueprintMapLibrary.Map_Find` (`self.As SBZPlayer Character_0`) (`Pawn.PlayerState` SBZPlayerCharacter)))
  ;[1 1 1] OnPlayerDealDamage
  (if _returnvalue
    (`/Game/Mods/_LesnovMods/KillCounter/UI_KillCount.OnPlayerDamage` _value Damage)))

(event `OnTakenDamage_Event_0`
  (params (DamageEventData :type "SBZDamageEvent Structure (by ref)"))
  (bind (_attacker _causer _victim _equippabledata _throwabledata _damage _armordamage _healthdamage _bcritical _bwasarmorbroken _biskillshot) (break `SBZDamageEvent` DamageEventData))
  ;[1 1 1] OnTakenDamage
  (bind _assbzplayer_character (cast `SBZPlayerCharacter` _attacker))
  (`self.OnPlayerDealDamage` _assbzplayer_character (`KismetMathLibrary.FTrunc` _damage))
  (if _biskillshot
    (`self.OnPlayerKill` _assbzplayer_character)))

(event `OnPlayerInEscapeChanged_Event_0`
  (params (PlayerInEscapeChangedEventData :type "SBZPlayerInEscapeChangedEvent Structure (by ref)"))
  ;[1 1 1] OnPlayerInEscapeChanged
  (if (== PlayerInEscapeChangedEventData_Inside PlayerInEscapeChangedEventData_Total)
    (`self.OnEscapeBoundReachedMaxPlayers`)))

(event `CustomEvent_0`
  ;[1 1 1] BeginPlay
  (bind _assbzplayer_character (`/Game/Mods/_LesnovMods/BML_Actor.ValidCheck(Wait | SBZPlayerCharacter)`))
  (`self.OnPlayerKill` _assbzplayer_character)
  (`KismetSystemLibrary.PrintString` (`KismetSystemLibrary.GetDisplayName` _assbzplayer_character))
  (`self.OnPlayerDealDamage` _assbzplayer_character (`KismetMathLibrary.RandomIntegerInRange` 0 550)))

(event `self.ReceiveBeginPlay`
  ;[1 1 1] BeginPlay
  (`parent.ReceiveBeginPlay`)
  (bind _savegame (`/Game/Mods/_LesnovMods/BML_Object.HandleSaveGame` "/Game/Mods/_LesnovMods/KillCounter/KillCounterSaveGame.KillCounterSaveGame_C" :!label _label)
    (:`Exec`
      (bind _askill_counter_save_game (cast `/Game/Mods/_LesnovMods/KillCounter/KillCounterSaveGame` _savegame)
        (:`then`
          (set `self.As Kill Counter Save Game` _askill_counter_save_game)
          (`/Game/Mods/_LesnovMods/BML_Actor.IsInEditor`
            (:`InEditor`
              (`self.CreateKillCounterHUD`)
              (`self.UpdateKillCountHUD`)
              (`KismetSystemLibrary.K2_SetTimerDelegate` (delegate `CustomEvent_0`) 1.0 true)
              (`self.EnableInput` (`GameplayStatics.GetPlayerController` 0))
              (`KismetSystemLibrary.Delay` 3.0))
            (:`InGame`
              (bind _assbzplayer_character (`/Game/Mods/_LesnovMods/BML_Actor.ValidCheck(Wait | SBZPlayerCharacter)` :!label _label_2))
              (set `self.As SBZPlayer Character` _assbzplayer_character)
              (`self.CreateKillCounterHUD`)
              (bind _returnvalue (`SBZEventLibrary.GetGameEventBroker`))
              (add `SBZGameEventBroker.OnTakenDamage` _returnvalue (`|CreateDelegate` :!event `OnTakenDamage_Event_0`))
              (add `SBZGameEventBroker.OnPlayerInEscapeChanged` _returnvalue (`|CreateDelegate` :!event `OnPlayerInEscapeChanged_Event_0`)) ; Execute when player enters escape bound box
              (`self.ObtainPlayers`)
              (`self.EnableInput` (`/Game/Mods/_LesnovMods/BML_Actor.GetLocalPlayerController(Comp)`)))))
        (:`CastFailed`
          (`KismetSystemLibrary.Delay` 1.0 :!label _label_3)
          (goto _label))))
    (:`Error`
      (goto _label_3))))

(event `OnDestroyed_Event_0`
  (params (DestroyedActor :type "Actor Object Reference"))
  ;[1 1 1] BeginPlay
  (goto _label_2))

(event `ObtainPlayers`
  (`KismetSystemLibrary.K2_SetTimer` null "UpdateKillCountHUD" 15.0 true))

(event `Key|K` :consume false
  (params (Key :type "Key Structure"))
  (:`Pressed`
    (`self.CreateKillCounterHUDMenu`)))

(event `OnEscapeBoundReachedMaxPlayers`
  ;[1 1 1] OnEscapeBoundReachedMaxPlayers(Executed when all players enter the escape bound) - Move the kill count HUD to the right buttom.
  (set `self.HUDOriginPos` (`KismetMathLibrary.Conv_Vector2DToVector` (`CanvasPanelSlot.GetPosition` (`WidgetLayoutLibrary.SlotAsCanvasSlot` (`/Game/Mods/_LesnovMods/KillCounter/Menu_KillCounter.ScaleBox_0` (`self.Menu_KillCounter`))))))
  (bind (_direction _newtrack_0) (`Timeline|Timeline_0` :!via `PlayFromStart`)
    (:`Update`
      (bind (_returnvalue_x _returnvalue_y) (`KismetMathLibrary.BreakVector` (`KismetMathLibrary.VLerp` (`self.HUDOriginPos`) (670.198669 289.240295 0.0) _newtrack_0)))
      (`CanvasPanelSlot.SetPosition` (`WidgetLayoutLibrary.SlotAsCanvasSlot` (`/Game/Mods/_LesnovMods/KillCounter/Menu_KillCounter.ScaleBox_0` (`self.Menu_KillCounter`))) (`KismetMathLibrary.MakeVector2D` _returnvalue_x _returnvalue_y)))))

(event `OnHudMenuOpen`
  ;[1 1 1] OnHudMenuOpen
  (`/Game/Mods/_LesnovMods/KillCounter/HudMenu_KillCounter.InitializeHudMenu` (`self.HudMenu`) (`self.As Kill Counter Save Game`))
  (`KismetSystemLibrary.Delay` 0.2)
  (set `PlayerController.bShowMouseCursor` true (`/Game/Mods/_LesnovMods/BML_Actor.GetLocalPlayerController(Comp)`)))

(event `OnHudMenuCreated`
  (bind _hudmenu (`self.HudMenu`))
  ;[1 1 1] OnHudMenuCreated
  (add `/Game/Mods/_LesnovMods/KillCounter/HudMenu_KillCounter.OnSaveButtonPressed` _hudmenu (delegate `OnSaved_Event_0`))
  (add `/Game/Mods/_LesnovMods/KillCounter/HudMenu_KillCounter.OnHideOtherPlayers` _hudmenu (delegate `OnHideOtherPlayers_Event_0`)))

(event `OnHideOtherPlayers_Event_0`
  (params (IsChecked :type Boolean))
  (bind _as_sbzplayer_character_0 (`self.As SBZPlayer Character_0`))
  ;[1 1 1] OnHudMenuCreated
  (bind _keys (`BlueprintMapLibrary.Map_Keys` _as_sbzplayer_character_0))
  (for _array_element _keys
    (if (!= (`Pawn.PlayerState` (`self.As SBZPlayer Character`)) _array_element)
      (bind (_value _returnvalue) (`BlueprintMapLibrary.Map_Find` _as_sbzplayer_character_0 _array_element))
      (if _returnvalue
        (`Widget.SetVisibility` _value (select `bool` IsChecked :`false` "SelfHitTestInvisible" :`true` "Collapsed" :!type "ESlateVisibility Enum"))))))

(event `OnPlayerDefeatStateChangedDelegate_Event_0`
  (params (InData :type "SBZPlayerDefeatStateChangedData Structure (by ref)"))
  ;[1 1 1] Might be better to use instead of OnDestroy later
  (if (and (`|EnumEquality` InData_OldDefeatState "InCustody") (== InData_PlayerState (`Pawn.PlayerState` (`self.As SBZPlayer Character`))))
    _))

(event `OnSaved_Event_0`
  (params (PositionOffset :type "Vector2D Structure") (ScaleOffset :type "Float (double-precision)") (HideName :type Boolean) (HideMiscText :type Boolean) (HideOtherPlayers :type Boolean))
  (bind _as_kill_counter_save_game (`self.As Kill Counter Save Game`))
  ;[1 1 1] OnHudMenuCreated
  (set `/Game/Mods/_LesnovMods/KillCounter/KillCounterSaveGame.PositionOffset` PositionOffset _as_kill_counter_save_game)
  (set `/Game/Mods/_LesnovMods/KillCounter/KillCounterSaveGame.ScaleOffset` ScaleOffset _as_kill_counter_save_game)
  (set `/Game/Mods/_LesnovMods/KillCounter/KillCounterSaveGame.HideName` HideName _as_kill_counter_save_game)
  (set `/Game/Mods/_LesnovMods/KillCounter/KillCounterSaveGame.HideMiscText` HideMiscText _as_kill_counter_save_game)
  (set `/Game/Mods/_LesnovMods/KillCounter/KillCounterSaveGame.HideOtherPlayers` HideOtherPlayers _as_kill_counter_save_game)
  (`/Game/Mods/_LesnovMods/BML_Object.SaveToSlot(Macro)` (`self.As Kill Counter Save Game`))
  (`Widget.SetVisibility` (`self.HudMenu`) "Collapsed")
  (set `PlayerController.bShowMouseCursor` false (`/Game/Mods/_LesnovMods/BML_Actor.GetLocalPlayerController(Comp)`)))

(fn `CreateKillCounterHUD`
  (bind _as_kill_counter_save_game (`self.As Kill Counter Save Game`))
  (bind _scalebox_0 (`/Game/Mods/_LesnovMods/KillCounter/Menu_KillCounter.ScaleBox_0` (`self.Menu_KillCounter`)))
  (bind (_positionoffset_x _positionoffset_y) (`KismetMathLibrary.BreakVector2D` (`/Game/Mods/_LesnovMods/KillCounter/KillCounterSaveGame.PositionOffset` _as_kill_counter_save_game)))
  (bind _scaleoffset (`/Game/Mods/_LesnovMods/KillCounter/KillCounterSaveGame.ScaleOffset` _as_kill_counter_save_game))
  (bind _returnvalue (`|CreateWidget` "/Game/Mods/_LesnovMods/KillCounter/Menu_KillCounter.Menu_KillCounter_C"))
  (`UserWidget.AddToViewport` _returnvalue 9999)
  (set `self.Menu_KillCounter` _returnvalue)
  (`CanvasPanelSlot.SetPosition` (`WidgetLayoutLibrary.SlotAsCanvasSlot` _scalebox_0) (`KismetMathLibrary.MakeVector2D` _positionoffset_x _positionoffset_y))
  (`ScaleBox.SetUserSpecifiedScale` _scalebox_0 _scaleoffset)
  (`KismetSystemLibrary.PrintString` (`KismetStringLibrary.Conv_DoubleToString` _scaleoffset) true true (struct :`R` 1.0 :`G` 0.028558 :`A` 1.0) 15.0))

(fn `CreateKillCounterHUDMenu`
  (`/Engine/EditorBlueprintResources/StandardMacros.IsValid` (`self.HudMenu`)
    (:`Is Valid`
      (if (`Widget.IsVisible` (`self.HudMenu`))
        (`Widget.SetVisibility` (`self.HudMenu`) "Collapsed")
        (set `PlayerController.bShowMouseCursor` false (`/Game/Mods/_LesnovMods/BML_Actor.GetLocalPlayerController(Comp)`))
        (else
          (`Widget.SetVisibility` (`self.HudMenu`) "SelfHitTestInvisible")
          (`self.OnHudMenuOpen` :!label _label))))
    (:`Is Not Valid`
      (bind _returnvalue (`|CreateWidget` "/Game/Mods/_LesnovMods/KillCounter/HudMenu_KillCounter.HudMenu_KillCounter_C" null (`self.Menu_KillCounter`)))
      (`UserWidget.AddToViewport` _returnvalue 9999)
      (set `self.HudMenu` _returnvalue)
      (`self.OnHudMenuCreated`)
      (goto _label))))

(fn `UpdateKillCountHUD`
  (locals (Local_SBZPlayerCharacter :type "SBZPlayerCharacter Object Reference") (Local_KillCount :type "/Game/Mods/_LesnovMods/KillCounter/UI_KillCount Object Reference"))
  (bind _as_kill_counter_save_game (`self.As Kill Counter Save Game`))
  (bind _playerstate (`Pawn.PlayerState` (`local.Local_SBZPlayerCharacter`)))
  (bind _outactors (`GameplayStatics.GetAllActorsOfClass` "/Script/Starbreeze.SBZPlayerCharacter"))
  (for _array_element _outactors
    (set `local.Local_SBZPlayerCharacter` _array_element)
    (if (`.ReturnValue` (`BlueprintMapLibrary.Map_Find` (`self.As SBZPlayer Character_0`) _playerstate))
      _
      (elif (`/Game/Mods/_LesnovMods/KillCounter/KillCounterSaveGame.HideOtherPlayers` (`self.As Kill Counter Save Game`))
        (if (== (`local.Local_SBZPlayerCharacter`) (`self.As SBZPlayer Character`))
          (bind _returnvalue (`|CreateWidget` "/Game/Mods/_LesnovMods/KillCounter/UI_KillCount.UI_KillCount_C" null (`KismetTextLibrary.Conv_StringToText` (`PlayerState.GetPlayerName` _playerstate)) :!label _label))
          (set `local.Local_KillCount` _returnvalue)
          (`PanelWidget.AddChild` (`/Game/Mods/_LesnovMods/KillCounter/Menu_KillCounter.VerticalBox_30` (`self.Menu_KillCounter`)) (`local.Local_KillCount`))
          (`BlueprintMapLibrary.Map_Add` (`self.As SBZPlayer Character_0`) (`Pawn.PlayerState` (`local.Local_SBZPlayerCharacter`)) (`local.Local_KillCount`))
          (`Widget.SetVisibility` (`/Game/Mods/_LesnovMods/KillCounter/UI_KillCount.PlayerName` (`local.Local_KillCount`)) (select `bool` (`/Game/Mods/_LesnovMods/KillCounter/KillCounterSaveGame.HideName` _as_kill_counter_save_game) :`false` "SelfHitTestInvisible" :`true` "Hidden" :!type "ESlateVisibility Enum"))
          (`Widget.SetVisibility` (`/Game/Mods/_LesnovMods/KillCounter/UI_KillCount.SizeBox_1` (`local.Local_KillCount`)) (select `bool` (`/Game/Mods/_LesnovMods/KillCounter/KillCounterSaveGame.HideMiscText` _as_kill_counter_save_game) :`false` "SelfHitTestInvisible" :`true` "Collapsed" :!type "ESlateVisibility Enum"))
          (`Widget.SetVisibility` (`/Game/Mods/_LesnovMods/KillCounter/UI_KillCount.SizeBox_0` (`local.Local_KillCount`)) (select `bool` (`/Game/Mods/_LesnovMods/KillCounter/KillCounterSaveGame.HideMiscText` _as_kill_counter_save_game) :`false` "SelfHitTestInvisible" :`true` "Collapsed" :!type "ESlateVisibility Enum")))
        (else
          (goto _label))))))

(fn `UserConstructionScript`
  (`parent.UserConstructionScript`))