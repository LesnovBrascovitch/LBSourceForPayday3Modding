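; Test mod actor that injects a cosmetic suit base into the game's suit database to check that cosmetic loading works.
; On BeginPlay it adds SuitBaseTesting to SuitDataBase's SuitBases, then puts a Menu_AddCosmetics widget on the viewport at a high Z-order.
; It then appends the display name of every suit base in the database to that menu's text field.
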(event `self.ReceiveBeginPlay`
  (`parent.ReceiveBeginPlay`)
  (`KismetArrayLibrary.Array_AddUnique` (`SBZSuitBaseDatabase.SuitBases` (`self.SuitDataBase`)) (`self.SuitBase_Testing`))
  (bind _returnvalue (`|CreateWidget` "/Game/Mods/_Testing/ConsmeticLoad/Menu_AddCosmetics.Menu_AddCosmetics_C"))
  (`UserWidget.AddToViewport` _returnvalue 9999)
  (set `self.NewVar_0` _returnvalue)
  (for _array_element (`SBZSuitBaseDatabase.SuitBases` (`self.SuitDataBase`))
    (`/Game/Mods/_LesnovMods/BML_Object.AddText` (`/Game/Mods/_Testing/ConsmeticLoad/Menu_AddCosmetics.EditableText_0` (`self.NewVar_0`)) (`KismetSystemLibrary.GetDisplayName` _array_element))))

(fn `UserConstructionScript`
  (`parent.UserConstructionScript`))